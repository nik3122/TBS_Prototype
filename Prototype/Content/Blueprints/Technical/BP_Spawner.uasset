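; Spawner actor that repeatedly creates instances of a given class around its own location for as long as it runs.
; BeginPlay and the Spawn timer event share one path, which spawns immediately and re-arms a one-shot timer with a random delay between the min and max times.
; Each spawn lands at the spawner's height, offset in X and Y by a random unit vector scaled by SpawnRadius, ignoring collisions.
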(event Custom|Spawn
  (bind _returnvalue (Math|Random|RandomUnitVector))
  (bind _self self)
  (bind _spawn_radius (Variables|Spawner|GetSpawn%20Radius))
  (bind _returnvalue_2 (* _returnvalue _spawn_radius))
  (bind _returnvalue_3 (Transformation|GetActorLocation _self))
  (bind _returnvalue_4 (+ _returnvalue_2 _returnvalue_3))
  (bind (_x _y) (Math|Vector|BreakVector _returnvalue_4))
  (Utilities|Time|SetTimerbyEvent (delegate Custom|Spawn) (Math|Random|RandomFloatinRange (Variables|Spawner|GetSpawnTimeMin) (Variables|Spawner|GetSpawnTimeMax)))
  (Game|SpawnActorfromClass (Variables|Spawner|GetClassToSpawn) (Math|Transform|MakeTransform (Math|Vector|MakeVector _x _y (.Z (Math|Vector|BreakVector _returnvalue_3))) "0, 0, 0" "1,1,1") "AlwaysSpawn" 0 0))

(event EventBeginPlay
  (bind _returnvalue (Math|Random|RandomUnitVector))
  (bind _self self)
  (bind _spawn_radius (Variables|Spawner|GetSpawn%20Radius))
  (bind _returnvalue_2 (* _returnvalue _spawn_radius))
  (bind _returnvalue_3 (Transformation|GetActorLocation _self))
  (bind _returnvalue_4 (+ _returnvalue_2 _returnvalue_3))
  (bind (_x _y) (Math|Vector|BreakVector _returnvalue_4))
  (Utilities|Time|SetTimerbyEvent (delegate Custom|Spawn) (Math|Random|RandomFloatinRange (Variables|Spawner|GetSpawnTimeMin) (Variables|Spawner|GetSpawnTimeMax)))
  (Game|SpawnActorfromClass (Variables|Spawner|GetClassToSpawn) (Math|Transform|MakeTransform (Math|Vector|MakeVector _x _y (.Z (Math|Vector|BreakVector _returnvalue_3))) "0, 0, 0" "1,1,1") "AlwaysSpawn" 0 0))

(fn ConstructionScript)