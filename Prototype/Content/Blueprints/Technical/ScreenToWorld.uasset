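; ScreenToWorld is a helper function set that converts the mouse cursor position into a world point and finds the map tile under it.
; IntersectCursorLinePlane deprojects the cursor and intersects that ray with a given plane, returning a zero vector if deprojection fails.
; GetTileUnderCursor runs this for the first player controller against a fixed, slightly raised horizontal plane and looks up the point in the supplied PassMap.
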(fn IntersectCursorLinePlane
  (params (PlayerController :type Player%20Controller%20Object%20Reference) (PlaneOrigin :type Vector) (PlaneNormal :type Vector))
  (bind (_worldlocation _worlddirection _returnvalue) (Game|Player|ConvertMouseLocationToWorldSpace PlayerController))
  (if _returnvalue
    (return (+ (* _worlddirection (.T (Class|KismetMathLibrary|LinePlaneIntersectionOriginNormal _worldlocation (+ _worldlocation _worlddirection) PlaneOrigin PlaneNormal))) _worldlocation))
    (else
      (return (Math|Vector|MakeVector 0.0 0.0 0.0)))))

(fn GetTileUnderCursor
  (params (PassMap :type Pass%20Map%20Object%20Reference))
  (return (Class|PassMap|GetTileinPositionWorld PassMap (CallFunction|IntersectCursorLinePlane (Game|GetPlayerController 0) "0, 0,20.000000" "0, 0,1.000000"))))