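; BP_GMCamp is a camp on the global map that holds the action blocks available there and an arena fight level.
; When active, Setup loads the blocks from the game mode's camps DataTable using the camp's object name as row name, printing an error if none matches.
; An inactive camp gets a single placeholder "Unactive camp" block instead.
; Getters expose the data, and TryGetActionBlock finds a block by ID.
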(event EventBeginPlay)

(fn ConstructionScript)

(fn GetArenaFightLevel
  (return (Variables|Unknown|GetArenaFightLevel)))

(fn GetActionBlocksMap
  (return (Variables|Unknown|GetCampActionBlocksMap)))

(fn Setup
  (bind _self self)
  (bind _returnvalue (Utilities|GetObjectName _self))
  (if (Variables|Unknown|GetIsActive)
    (bind _table (Class|IBPGlobalMapManager|GetCampsDataTable(Message) (Game|GetGameMode)))
    (bind _returnvalue_2 (Utilities|GetDataTableRow _table (Utilities|String|StringToName _returnvalue))
      (:then
        (Variables|Unknown|SetCampActionBlocksMap _returnvalue_2))
      (:RowNotFound
        (Development|PrintString (Utilities|String|Append "ERROR: No suitable camp data was found for \"" _returnvalue "\"! Check the next asset: " (Class|KismetSystemLibrary|GetPathName _table)) true true "(R=1.000000,G=0.000000,B=0.000000,A=1.000000)" 5.0)))
    (else
      (Utilities|Array|Clear (.actionblocks (Variables|Unknown|GetCampActionBlocksMap)))
      (Utilities|Array|Add (.actionblocks (Variables|Unknown|GetCampActionBlocksMap)) (Utilities|Struct|MakeSTRC_ActionBlock "None" "Unactive camp" "/Engine/EngineMaterials/BlendFunc_DefBlend.BlendFunc_DefBlend" "This camp was deactivated." (Utilities|Array|MakeArray) false)))))

(fn TryGetActionBlock
  (params (ActionBlockID :type Name%20%28by%20ref%29))
  (for (_array_element _array_index) (.actionblocks (Variables|Unknown|GetCampActionBlocksMap))
    (if (Utilities|Name|Equal(Name) ActionBlockID (.ID (Utilities|Struct|BreakSTRC_ActionBlock _array_element)))
      (return true _array_element _array_index)))
  (return false "" -1))