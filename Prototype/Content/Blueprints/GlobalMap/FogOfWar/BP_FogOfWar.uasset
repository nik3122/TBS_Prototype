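; Fog of war actor for the global map that paints world-space markers into the FogOfWarAlpha render target.
; BeginPlay publishes its bounds' min corner and size to MCOL_Global as FOW_Pos_Size.
; DrawMarker stamps a dynamic brush material, converting marker center and extent to bounds-relative values with X/Y swapped and one axis flipped.
; EndPlay clears the target to black; the sample DrawMarker calls in the graph are unconnected.
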(event EventBeginPlay
  (bind (_origin _boxextent) (Collision|GetActorBounds false))
  (Rendering|Material|SetVectorParameterValue "/Game/Objects/MCOL_Global.MCOL_Global" "FOW_Pos_Size" (Utilities|Struct|MakeLinearColor (- (.x _origin) (.x _boxextent)) (- (.y _origin) (.y _boxextent)) (* (.x _boxextent) 2.0) (* (.y _boxextent) 2.0)) :!class /Script/Engine.KismetMaterialLibrary))

(event Collision|EventActorBeginOverlap
  (params (OtherActor :type Actor%20Object%20Reference)))

(event EventEndPlay
  (params (EndPlayReason :type EEndPlayReason%20Enum :default "Destroyed"))
  (Rendering|ClearRenderTarget2D (Variables|Default|GetFogOfWarAlpha)))

(fn ConstructionScript
  (bind _returnvalue (Rendering|Material|CreateDynamicMaterialInstance "/Game/Blueprints/GlobalMap/FogOfWar/MAT_FogOfWarBrush.MAT_FogOfWarBrush" "None" :!class /Script/Engine.KismetMaterialLibrary))
  (Variables|Default|SetBrushMaterial _returnvalue))

(fn DrawMarker
  (params (MarkerCenter :type Vector) (MarkerExtent :type Vector))
  (Rendering|Material|SetVectorParameterValue (Variables|Default|GetBrushMaterial) "RelativeSizeAndPos" (CallFunction|GetBrushSizeandPos MarkerCenter MarkerExtent) :!class /Script/Engine.MaterialInstanceDynamic)
  (Rendering|DrawMaterialtoRenderTarget (Variables|Default|GetFogOfWarAlpha) (Variables|Default|GetBrushMaterial)))

(fn GetBrushSizeandPos
  (params (MarkerCenter :type Vector) (MarkerExtent :type Vector))
  (bind (_origin _boxextent) (Collision|GetActorBounds false))
  (LocalVariables|SetLMarkerCenter (Math|Conversions|ToVector2D(Vector) MarkerCenter))
  (LocalVariables|SetLMarkerExtent (Math|Conversions|ToVector2D(Vector) MarkerExtent))
  (LocalVariables|SetLFogCenter (Math|Conversions|ToVector2D(Vector) _origin))
  (LocalVariables|SetLFogExtent (Math|Conversions|ToVector2D(Vector) _boxextent))
  (return (Math|Color|MakeColor (.x (/ (LocalVariables|GetLMarkerExtent) (LocalVariables|GetLFogExtent))) (.y (/ (LocalVariables|GetLMarkerExtent) (LocalVariables|GetLFogExtent))) (.x (/ (Math|Vector2D|MakeVector2D (- (.y (LocalVariables|GetLMarkerCenter)) (- (.y (LocalVariables|GetLFogCenter)) (.y (LocalVariables|GetLFogExtent)))) (- (+ (.x (LocalVariables|GetLFogCenter)) (.x (LocalVariables|GetLFogExtent))) (.x (LocalVariables|GetLMarkerCenter)))) (* (LocalVariables|GetLFogExtent) 2.0))) (.y (/ (Math|Vector2D|MakeVector2D (- (.y (LocalVariables|GetLMarkerCenter)) (- (.y (LocalVariables|GetLFogCenter)) (.y (LocalVariables|GetLFogExtent)))) (- (+ (.x (LocalVariables|GetLFogCenter)) (.x (LocalVariables|GetLFogExtent))) (.x (LocalVariables|GetLMarkerCenter)))) (* (LocalVariables|GetLFogExtent) 2.0))))))