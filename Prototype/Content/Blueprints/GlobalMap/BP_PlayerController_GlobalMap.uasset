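; Player controller for the global map that drives a top-down free camera.
; On BeginPlay it spawns the camera actor, makes it the view target, sets zoom pitch and arm-length limits, places it at the controlled pawn and calls TrackActor with MpGMPawn.
; Axis inputs zoom the spring arm, rotate yaw and move the camera along its forward and right vectors, scaled by speed variables rather than delta time.
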(event EventBeginPlay
  (Utilities|FlowControl|Sequence
    (:then_0
      (bind _returnvalue (Game|SpawnActorfromClass "/Game/Blueprints/Technical/BP_TopDownFreeCamera.BP_TopDownFreeCamera_C" (Math|Transform|MakeTransform "0, 0, 0" "0, 0, 0" "1,1,1") "AlwaysSpawn" self 0))
      (bind _output_get (Variables|Default|SetTopDownFreeCamera _returnvalue))
      (Game|Player|SetViewTargetwithBlend _output_get 0.0 "VTBlend_Linear" 0.0 false)
      (Default|SetMinMaxValues (Variables|Default|GetTopDownFreeCamera) 6e+01 5e+02 89.0 3e+03)
      (Transformation|SetActorLocation (Variables|Default|GetTopDownFreeCamera) (Transformation|GetActorLocation (Pawn|GetControlledPawn)) false false)
      (Default|TrackActor (Variables|Default|GetTopDownFreeCamera) (Variables|Default|GetmpGMPawn)))))

(event Input|AxisEvents|InputAxisWheel
  (params (AxisValue :type Float%20%28single-precision%29))
  (Default|ChangeSpringArmLength (Variables|Default|GetTopDownFreeCamera) (* AxisValue (Variables|Default|GetCameraZoomSpeed))))

(event Input|AxisEvents|InputAxisMoveX
  (params (AxisValue :type Float%20%28single-precision%29))
  (bind _topdownfreecamera (Variables|Default|GetTopDownFreeCamera))
  (bind _invalue (Utilities|IsZero AxisValue)
    (:NonZero
      (Transformation|SetActorLocation _topdownfreecamera (+ (* (* (Transformation|GetActorForwardVector (Variables|Default|GetTopDownFreeCamera)) (Variables|Default|GetDummySpeed)) _invalue) (Transformation|GetActorLocation _topdownfreecamera)) false false))))

(event Input|AxisEvents|InputAxisChangeCameraYawLeft
  (params (AxisValue :type Float%20%28single-precision%29))
  (bind _invalue (Utilities|IsZero AxisValue)
    (:NonZero
      (Default|ChangeYaw (Variables|Default|GetTopDownFreeCamera) (* _invalue (Variables|Default|GetCameraYawSpeed))))))

(event Input|AxisEvents|InputAxisChangeCameraYawRight
  (params (AxisValue :type Float%20%28single-precision%29))
  (bind _invalue (Utilities|IsZero AxisValue)
    (:NonZero
      (Default|ChangeYaw (Variables|Default|GetTopDownFreeCamera) (* _invalue (- 0.0 (Variables|Default|GetCameraYawSpeed)))))))

(event Input|AxisEvents|InputAxisMoveY
  (params (AxisValue :type Float%20%28single-precision%29))
  (bind _topdownfreecamera (Variables|Default|GetTopDownFreeCamera))
  (bind _invalue (Utilities|IsZero AxisValue)
    (:NonZero
      (Transformation|SetActorLocation _topdownfreecamera (+ (* (* (Transformation|GetActorRightVector (Variables|Default|GetTopDownFreeCamera)) (Variables|Default|GetDummySpeed)) _invalue) (Transformation|GetActorLocation _topdownfreecamera)) false false))))

(fn ConstructionScript)