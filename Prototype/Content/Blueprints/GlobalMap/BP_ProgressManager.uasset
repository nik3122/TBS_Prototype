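; Progress manager for the global map that stores, changes and tests named progress variables used to track game state.
; Values resolve from a map of active overrides first, falling back to defaults in a data table supplied through Setup.
; Changes set or add to a value and fire a changed event, while checks compare against a value, singly or AND-combined.
; Only the overrides are saved, as parallel name and value arrays.
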(fn CheckProgressVariable
  (params (CheckProgressVariable :type STRC%20Check%20Progress%20Variable%20Structure))
  (bind (_doesvariableexist _value) (CallFunction|GetProgressVariableValue (.progressvariable CheckProgressVariable)))
  (LocalVariables|SetLCheckValue (.value CheckProgressVariable))
  (LocalVariables|SetLValue _value)
  (if _doesvariableexist
    (switch Utilities|FlowControl|Switch|SwitchonENUM_Compare (.condition CheckProgressVariable)
      (:NewEnumerator0
        (return (< (LocalVariables|GetLValue) (LocalVariables|GetLCheckValue)) true))
      (:NewEnumerator1
        (return (<= (LocalVariables|GetLValue) (LocalVariables|GetLCheckValue)) true))
      (:NewEnumerator2
        (return (== (LocalVariables|GetLValue) (LocalVariables|GetLCheckValue)) true))
      (:NewEnumerator3
        (return (>= (LocalVariables|GetLValue) (LocalVariables|GetLCheckValue)) true))
      (:NewEnumerator4
        (return (> (LocalVariables|GetLValue) (LocalVariables|GetLCheckValue)) true)))
    (else
      (Development|PrintString 0 (Utilities|String|Append "ERROR: Trying to check progress variable \"" (Utilities|String|ToString(Name) (.progressvariable CheckProgressVariable)) "\" which doesn't exist!") true true "(R=1.000000,G=0.000000,B=0.000000,A=1.000000)" 5.0)
      (return false false))))

(fn ChangeProgressVariable
  (params (ChangeProgressVariable :type STRC%20Change%20Progress%20Variable%20Structure))
  (bind (_doesvariableexist _value) (CallFunction|GetProgressVariableValue (.progressvariable ChangeProgressVariable)))
  (LocalVariables|SetLOldValue _value)
  (if _doesvariableexist
    (Utilities|FlowControl|Sequence
      (:then_0
        (switch Utilities|FlowControl|Switch|SwitchonENUM_ProgressVariableOperation (.operation ChangeProgressVariable)
          (:NewEnumerator0
            (LocalVariables|SetLNewValue (.value ChangeProgressVariable)))
          (:NewEnumerator1
            (LocalVariables|SetLNewValue (+ (.value ChangeProgressVariable) (LocalVariables|GetLOldValue))))))
      (:then_1
        (Utilities|Map|Add (Variables|Default|GetActiveProgressVariables) (.progressvariable ChangeProgressVariable) (LocalVariables|GetLNewValue))
        (Default|CallEventProgressVariableChanged (.progressvariable ChangeProgressVariable) (LocalVariables|GetLOldValue) (LocalVariables|GetLNewValue))
        (return true)))
    (else
      (return false))))

(fn GetProgressVariableValue
  (params (ProgressVariableName :type Name))
  (bind _activeprogressvariables (Variables|Default|GetActiveProgressVariables))
  (bind (_value _returnvalue) (Utilities|Map|Find _activeprogressvariables ProgressVariableName))
  (if _returnvalue
    (return true _value)
    (else
      (bind _returnvalue_2 (Utilities|GetDataTableRow (Variables|Default|GetProgressVariablesTable) ProgressVariableName)
        (:then
          (return true (Utilities|Struct|BreakSTRC_ProgressVariable _returnvalue_2)))
        (:RowNotFound
          (Development|PrintString 0 (Utilities|String|Append "ERROR: Progress variable \"" (Utilities|String|ToString(Name) ProgressVariableName) "\" is not found!") true true "(R=1.000000,G=0.000000,B=0.000000,A=1.000000)" 5.0)
          (return false 0))))))

(fn Setup
  (params (ProgressVariablesTable :type Data%20Table%20Object%20Reference))
  (Variables|Default|SetProgressVariablesTable ProgressVariablesTable))

(fn SaveState
  (bind _activeprogressvariables (Variables|Default|GetActiveProgressVariables))
  (bind _keys (Utilities|Map|Keys _activeprogressvariables))
  (bind _values (Utilities|Map|Values _activeprogressvariables))
  (return (Utilities|Struct|MakeSTRC_ProgressManagerState _keys _values)))

(fn LoadState
  (params (State :type STRC%20Progress%20Manager%20State%20Structure%20%28by%20ref%29))
  (Utilities|Map|Clear (Variables|Default|GetActiveProgressVariables))
  (for (_array_element _array_index) (.activeprogressvariablesnames State)
    (Utilities|Map|Add (Variables|Default|GetActiveProgressVariables) _array_element (Utilities|Array|Get(acopy) (.activeprogressvariablesvalues State) _array_index))))

(fn MultiCheckProgressVariable
  (params (ProgressVariableChecks :type Array%20of%20STRC%20Check%20Progress%20Variable%20Structures))
  ;[1 0.4074 0] AND logics: if only a single check fails - all of them fail:
  (for _array_element ProgressVariableChecks
    (if (not (.IsTrue (CallFunction|CheckProgressVariable _array_element)))
      (return false)))
  (return true))