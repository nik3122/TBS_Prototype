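; Global map road actor that shows its spline-built road on cursor hover while active and available.
; Construction rebuilds one spline mesh per point-to-point segment, with point-driven scale, distance-based material tiling and offset, and an outline stencil value.
; Meshes start hidden at BeginPlay; availability changes play optional open or close level sequences through a MEMLEAK macro.
; Equal-length segmentation and custom-depth highlight toggling exist only as unconnected logic.
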(event EventOnSetAvailable
  (if (Class|SourceControlHelpers|IsAvailable)
    (Utilities|IsValid (Variables|Default|GetSequenceOnOpen)
      (:Is%20Valid
        (Utilities|MEMLEAK
          (:Out
            (bind _returnvalue (Sequencer|Player|CreateLevelSequencePlayer self (Variables|Default|GetSequenceOnOpen) (Utilities|Struct|MakeMovieSceneSequencePlaybackSettings false "(Value=0)" 1.0 0.0 false false false false false false false true)))
            (Sequencer|Player|Play _returnvalue :!class /Script/MovieScene.MovieSceneSequencePlayer)))))
    (else
      (Utilities|IsValid (Variables|Default|GetSequenceOnClose)
        (:Is%20Valid
          (Utilities|MEMLEAK
            (:Out
              (bind _returnvalue_2 (Sequencer|Player|CreateLevelSequencePlayer self (Variables|Default|GetSequenceOnClose) (Utilities|Struct|MakeMovieSceneSequencePlaybackSettings false "(Value=0)" 1.0 0.0 false false false false false false false true)))
              (Sequencer|Player|Play _returnvalue_2 :!class /Script/MovieScene.MovieSceneSequencePlayer))))))))

(event EventBeginPlay
  (for _array_element (Variables|Default|GetSplineMeshComponents)
    (Rendering|SetVisibility _array_element false true)))

(event MouseInput|EventActorBeginCursorOver
  ;[1 1 1] Should be transfered into c++ with binding/unbinding on activation/deactivation for the performance.
  (if (and (Variables|Default|GetmIsActive) (Variables|Default|GetmIsAvailable))
    (Rendering|SetVisibility (Variables|Default|GetmpRoadSpline) true true)))

(event MouseInput|EventActorEndCursorOver
  ;[1 1 1] Should be transfered into c++ with binding/unbinding on activation/deactivation for the performance.
  (Rendering|SetVisibility (Variables|Default|GetmpRoadSpline) false true))

(fn ConstructionScript
  (|CallParentFunction)
  (Utilities|FlowControl|Sequence
    (:then_0
      (CallFunction|GenerateMeshes))))

(fn GenerateMeshes
  (Utilities|FlowControl|Sequence
    (:then_0
      (Utilities|Array|Clear (Variables|Default|GetSplineMeshComponents)))
    (:then_1
      (for _array_element (Components|GetChildrenComponents (Variables|Default|GetmpRoadSpline) true)
        (Components|DestroyComponent _array_element)))
    (:then_2
      ;[1 1 1] Generate meshes by Spline Points
      (for _index (range 0 (- (Spline|GetNumberOfSplinePoints (Variables|Default|GetmpRoadSpline)) 2))
        (LocalVariables|SetLCurrentIndex _index)
        (bind _returnvalue (AddComponent|AddSplineMeshComponent true))
        (bind _output_get (LocalVariables|SetLMesh _returnvalue))
        (Utilities|Array|Add (Variables|Default|GetSplineMeshComponents) _output_get)
        (Transformation|AttachComponentToComponent (LocalVariables|GetLMesh) (Variables|Default|GetmpRoadSpline) "None" "KeepRelative" "KeepRelative" "KeepRelative" false)
        (Rendering|SetCustomDepthStencilValue (LocalVariables|GetLMesh) (Variables|Default|GetPostFXRoadOutlineBitMask))
        (LocalVariables|SetLNextIndex (+ 1 (LocalVariables|GetLCurrentIndex)))
        (SplineMesh|SetStartandEnd (LocalVariables|GetLMesh) (.Location (Spline|GetLocationandTangentatSplinePoint (Variables|Default|GetmpRoadSpline) (LocalVariables|GetLCurrentIndex) "Local")) (.Tangent (Spline|GetLocationandTangentatSplinePoint (Variables|Default|GetmpRoadSpline) (LocalVariables|GetLCurrentIndex) "Local")) (.Location (Spline|GetLocationandTangentatSplinePoint (Variables|Default|GetmpRoadSpline) (LocalVariables|GetLNextIndex) "Local")) (.Tangent (Spline|GetLocationandTangentatSplinePoint (Variables|Default|GetmpRoadSpline) (LocalVariables|GetLNextIndex) "Local")) true :!class /Script/Engine.SplineMeshComponent)
        (SplineMesh|SetStartScale (LocalVariables|GetLMesh) (Math|Vector2D|MakeVector2D (.y (* (Spline|GetScaleatSplinePoint (Variables|Default|GetmpRoadSpline) (LocalVariables|GetLCurrentIndex)) (Variables|Default|GetScaleMultiplier))) (.z (* (Spline|GetScaleatSplinePoint (Variables|Default|GetmpRoadSpline) (LocalVariables|GetLCurrentIndex)) (Variables|Default|GetScaleMultiplier)))) true :!class /Script/Engine.SplineMeshComponent)
        (SplineMesh|SetEndScale (LocalVariables|GetLMesh) (Math|Vector2D|MakeVector2D (.y (* (Spline|GetScaleatSplinePoint (Variables|Default|GetmpRoadSpline) (LocalVariables|GetLNextIndex)) (Variables|Default|GetScaleMultiplier))) (.z (* (Spline|GetScaleatSplinePoint (Variables|Default|GetmpRoadSpline) (LocalVariables|GetLNextIndex)) (Variables|Default|GetScaleMultiplier)))) true :!class /Script/Engine.SplineMeshComponent)
        (Rendering|Material|SetScalarParameterValueonMaterials (LocalVariables|GetLMesh) "UTiling" (/ (- (Spline|GetDistanceAlongSplineatSplinePoint (Variables|Default|GetmpRoadSpline) (LocalVariables|GetLNextIndex)) (Spline|GetDistanceAlongSplineatSplinePoint (Variables|Default|GetmpRoadSpline) (LocalVariables|GetLCurrentIndex))) (Variables|Default|GetUnitTilingByLength)))
        (Rendering|Material|SetScalarParameterValueonMaterials (LocalVariables|GetLMesh) "UOffset" (/ (Spline|GetDistanceAlongSplineatSplinePoint (Variables|Default|GetmpRoadSpline) (LocalVariables|GetLCurrentIndex)) (Variables|Default|GetUnitTilingByLength)))))))