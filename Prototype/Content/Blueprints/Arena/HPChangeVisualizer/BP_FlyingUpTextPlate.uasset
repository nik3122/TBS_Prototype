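; Floating text plate actor in the arena's HP change visualizer that shows a colored text rising from a given position.
; SetupAndPlay moves it to the start point, sets the text render's color and string, unhides it and starts the lifetime timer.
; While active, Tick moves it straight up at constant speed, then hides and deactivates it when time runs out.
; It starts hidden and is never destroyed, so the same instance can be replayed.
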(event EventBeginPlay
  (Variables|Default|SetVelocity (Math|Vector|MakeVector 0.0 0.0 (Variables|Default|GetSpeed)))
  (Rendering|SetActorHiddenInGame true))

(event EventTick
  (params (DeltaSeconds :type Float%20%28single-precision%29))
  (if (Variables|Default|GetIsActive)
    (Transformation|SetActorLocation (+ (Transformation|GetActorLocation) (* (Variables|Default|GetVelocity) DeltaSeconds)) false false)
    (Variables|Default|SetTimer (- (Variables|Default|GetTimer) DeltaSeconds))
    (if (> 0.0 (Variables|Default|GetTimer))
      (Rendering|SetActorHiddenInGame true)
      (Variables|Default|SetIsActive false))))

(fn ConstructionScript)

(fn SetupandPlay
  (params (StartingPosition :type Vector) (TextColor :type Color%20Structure) (Text :type String))
  (Transformation|SetActorLocation StartingPosition false false)
  (Variables|Default|SetTimer (Variables|Default|GetLifeTime))
  (Rendering|Components|TextRender|SetTextRenderColor (Variables|Default|GetTextRender) TextColor)
  (Rendering|Components|TextRender|SetText (Variables|Default|GetTextRender) (Utilities|Text|ToText(String) Text))
  (Rendering|SetActorHiddenInGame false)
  (Variables|Default|SetIsActive true))