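; Widget component that shows an actor's 3D HP bar and floating HP change numbers in the arena.
; On non-dedicated-server BeginPlay it binds to the owner's damageable HP, death and revive events and pre-spawns a pool of flying text plates.
; HP changes reuse plates round-robin at random offsets, colored by sign.
; Tick polls HP and party color into the bar; death hides the component, revive shows it.
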(event Custom|OnHPChanged
  (params (pDamageable :type Damageable%20Object%20Reference) (deltaHP :type Integer) (dealer :type Actor%20Object%20Reference))
  (CallFunction|LaunchTextPlate deltaHP))

(event EventBeginPlay
  ;[1 0 0] DOESN'T CONSTRUCT WIDGET!!! or  isn't called...
  (|CallParentFunction)
  (if (not (Networking|IsDedicatedServer))
    (bind _returnvalue (Class|ArenaUnitInterface|GetVisualDamageable(Message) (Components|GetOwner)))
    (Variables|Default|SetOwnerDamageable _returnvalue)
    (Utilities|FlowControl|Sequence
      (:then_0
        (for _index (range 1 (Variables|Default|GetTextPlatesNumber))
          (bind _returnvalue_2 (Game|SpawnActorfromClass "/Game/Blueprints/Arena/HPChangeVisualizer/BP_FlyingUpTextPlate.BP_FlyingUpTextPlate_C" (Math|Transform|MakeTransform "0, 0, 0" "0, 0, 0" "1,1,1") "AlwaysSpawn" 0 0))
          (Utilities|Array|Add (Variables|Default|GetTextPlates) _returnvalue_2)))
      (:then_1
        (EventDispatchers|BindEventtoMEventHPChanged (Variables|Default|GetOwnerDamageable) (EventDispatchers|CreateEvent :!event Custom|OnHPChanged))
        (EventDispatchers|BindEventtoMEventDeath (Variables|Default|GetOwnerDamageable) (EventDispatchers|CreateEvent :!event OnDeath))
        (EventDispatchers|BindEventtoMEventRevive (Variables|Default|GetOwnerDamageable) (EventDispatchers|CreateEvent :!event OnRevive))))))

(event EventTick
  (params (DeltaSeconds :type Float%20%28single-precision%29))
  (CallFunction|UpdateHPBar))

(fn LaunchTextPlate
  (params (DeltaHP :type Integer))
  (LocalVariables|SetHPChange DeltaHP)
  (Utilities|FlowControl|Sequence
    (:then_0
      (LocalVariables|SetText (Utilities|String|ToString(Integer) (LocalVariables|GetHPChange)))
      (if (> 0 (LocalVariables|GetHPChange))
        (LocalVariables|SetColor (Math|Color|MakeColor 0 0 255 0))
        (else
          (LocalVariables|SetText (Utilities|String|Append "+" (LocalVariables|GetText)))
          (LocalVariables|SetColor (Math|Color|MakeColor 0 255 0 0)))))
    (:then_1
      (LocalVariables|SetTextPlate (Utilities|Array|Get(acopy) (Variables|Default|GetTextPlates) (Variables|Default|GetCurrentPlateIndex)))
      (bind _result (Math|Integer|IncrementInt (Variables|Default|GetCurrentPlateIndex))
        (:%20%20
          (Variables|Default|SetCurrentPlateIndex (Math|Integer|%(Integer) _result (Utilities|Array|Length (Variables|Default|GetTextPlates)))))))
    (:then_2
      (Default|SetupandPlay (LocalVariables|GetTextPlate) (+ (Transformation|GetWorldLocation) (* (Math|Random|RandomUnitVector) (Variables|Default|GetRandomOffsetRadius))) (LocalVariables|GetColor) (LocalVariables|GetText)))))

(fn UpdateHPBar
  (bind _ownerdamageable (Variables|Default|GetOwnerDamageable))
  (bind _returnvalue (Class|Damageable|GetCurrentMaxHP _ownerdamageable))
  (bind _returnvalue_2 (Class|Damageable|GetCurrentHP _ownerdamageable))
  (Utilities|IsValid (Variables|Default|GetOwnerDamageable)
    (:Is%20Valid
      (bind _asui_hpbar_3d (Utilities|Casting|CastToUI_HPBar3D (UserInterface|GetUserWidgetObject)))
      (Default|SetHP _asui_hpbar_3d _returnvalue_2 _returnvalue (/ (Math|Conversions|ToFloat(Integer) _returnvalue_2) (Math|Conversions|ToFloat(Integer) _returnvalue)))
      (bind _returnvalue_3 (Class|ArenaUnitInterface|GetSocialComponent(Message) (Components|GetOwner)))
      (Utilities|IsValid (Class|SocialComponent|GetParty _returnvalue_3)
        (:Is%20Valid
          (Default|SetSolidColor (Variables|/Game/Blueprints/Arena/HPChangeVisualizer/UI_HPBar3D.UI_HPBar3D_C|GetHPBar _asui_hpbar_3d) (.mpartycolor (Class|Party|GetPartyInfo (Class|SocialComponent|GetParty _returnvalue_3)))))))))

(fn SetIsFocused
  (params (IsFocused :type Boolean))
  (bind _asui_hpbar_3d (Utilities|Casting|CastToUI_HPBar3D (UserInterface|GetUserWidgetObject)))
  (Default|SetIsFocused _asui_hpbar_3d IsFocused))

(fn OnDeath
  (params (pDamageable :type Damageable%20Object%20Reference))
  (Rendering|SetVisibility false false))

(fn OnRevive
  (params (pDamageable :type Damageable%20Object%20Reference))
  (Rendering|SetVisibility true false))