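; Arena status effect that slows its target's tiled movement while active.
; Setup caches the target actor's tiled movement component; activation subtracts SpeedChange from its tile speed bonus and deactivation adds it back.
; Reactivation adds the new duration to the effect's own duration and keeps the current stage, so repeat applications extend the slow without deepening it.
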(event EventActivateInner
  (params (stage :type Integer))
  (bind _targetmovement (Variables|Default|GetTargetMovement))
  (Class|TiledMovement|SetTileSpeedBonus _targetmovement (- (Class|TiledMovement|GetTileSpeedBonus _targetmovement) (Variables|Default|GetSpeedChange))))

(event EventSetupInner
  (bind _returnvalue (Class|ArenaUnitInterface|GetTiledMovement(Message) (Variables|Default|GetmpTargetActor)))
  (Variables|Default|SetTargetMovement _returnvalue))

(event EventDeactivateInner
  (bind _targetmovement (Variables|Default|GetTargetMovement))
  (Class|TiledMovement|SetTileSpeedBonus _targetmovement (+ (Class|TiledMovement|GetTileSpeedBonus _targetmovement) (Variables|Default|GetSpeedChange))))

(fn ConstructionScript)

(fn ReactivateInner
  (params (duration :type Integer) (stage :type Integer))
  (return (+ duration (Class|StatusEffect|GetDuration)) (Variables|Default|GetmStage)))