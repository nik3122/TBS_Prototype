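; Hive status effect for the arena that damages its target and carries a visual that follows it.
; Each apply deals the effect's damage through the target's damageable interface and resets the turn timer to a huge value, so it is effectively permanent.
; Reactivation likewise returns a very long duration at a fixed first stage.
; A bound hive visual tracks the target actor and is destroyed on deactivation.
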(event EventDeactivateInner
  (Actor|DestroyActor (Variables|Default|GetHiveVisual)))

(event EventApplyInner
  (Variables|Default|SetmTurnsTimer 99999)
  (bind _returnvalue (Class|ArenaUnitInterface|GetDamageable(Message) (Variables|Default|GetmpTargetActor)))
  (Class|Damageable|Damage _returnvalue (Variables|Default|GetDamage)))

(event EventActivateInner
  (params (stage :type Integer)))

(fn ConstructionScript)

(fn ReactivateInner
  (params (duration :type Integer) (stage :type Integer))
  (return 9999 1))

(fn BindHiveVisual
  (params (HiveVisual :type BP%20Hive%20Visual%20Object%20Reference))
  (bind _output_get (Variables|Default|SetHiveVisual HiveVisual))
  (Default|SetFollowTarget _output_get (Variables|Default|GetmpTargetActor)))