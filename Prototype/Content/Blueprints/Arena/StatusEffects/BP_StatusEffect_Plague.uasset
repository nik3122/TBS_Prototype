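; Plague status effect for arena units that lowers the target's reaction rate and damage resistance while active.
; Setup caches the target's action manager and damageable through ArenaUnit_Interface.
; Activation subtracts a floored fraction of nominal reaction rate and a fixed resist amount from the target's bonuses, and deactivation adds both back.
; Reactivation adds the new duration to the current one and keeps the existing stage.
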(event EventActivateInner
  (params (stage :type Integer))
  (bind _targetactionmanager (Variables|Default|GetTargetActionManager))
  (bind _targetdamageable (Variables|Default|GetTargetDamageable))
  (Variables|Default|SetChangedReaction (Math|Float|Floor (* (Class|ActionManager|GetNominalReactionRate _targetactionmanager) (Variables|Default|GetReactionChange_S1))))
  (Class|ActionManager|SetReactionRateBonus _targetactionmanager (- (Class|ActionManager|GetReactionRateBonus _targetactionmanager) (Variables|Default|GetChangedReaction)))
  (Class|Damageable|SetResistBonus _targetdamageable (Class|DamageOperator|DamageSubtractDamage (Class|Damageable|GetResistBonus _targetdamageable) (Variables|Default|GetResistBonus_S1))))

(event EventSetupInner
  (bind _asarena_unit_interface (Utilities|Casting|CastToArenaUnit_Interface (Variables|Default|GetmpTargetActor)))
  (Utilities|FlowControl|Sequence
    (:then_0
      (bind _returnvalue (Class|ArenaUnitInterface|GetActionManager _asarena_unit_interface))
      (Variables|Default|SetTargetActionManager _returnvalue))
    (:then_1
      (bind _returnvalue_2 (Class|ArenaUnitInterface|GetDamageable _asarena_unit_interface))
      (Variables|Default|SetTargetDamageable _returnvalue_2))))

(event EventDeactivateInner
  (bind _targetactionmanager (Variables|Default|GetTargetActionManager))
  (bind _targetdamageable (Variables|Default|GetTargetDamageable))
  (Class|ActionManager|SetReactionRateBonus _targetactionmanager (+ (Class|ActionManager|GetReactionRateBonus _targetactionmanager) (Variables|Default|GetChangedReaction)))
  (Class|Damageable|SetResistBonus _targetdamageable (Class|DamageOperator|DamageAddDamage (Class|Damageable|GetResistBonus _targetdamageable) (Variables|Default|GetResistBonus_S1))))

(fn ConstructionScript)

(fn ReactivateInner
  (params (duration :type Integer) (stage :type Integer))
  (return (+ duration (Class|StatusEffect|GetDuration)) (Variables|Default|GetmStage)))