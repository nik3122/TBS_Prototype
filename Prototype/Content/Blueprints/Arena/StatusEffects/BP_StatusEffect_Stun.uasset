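; Stun status effect for the arena that marks its target's tiled movement as stunned while active.
; Setup caches the target's tiled movement and skeletal mesh through message calls on the actor.
; Activation sets the stun and attaches a Niagara effect to a mesh socket; deactivation clears both.
; Reactivation adds the incoming duration to the effect's own duration and keeps its current stage.
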(event EventSetupInner
  (Utilities|FlowControl|Sequence
    (:then_0
      (bind _returnvalue (Class|ArenaUnitInterface|GetTiledMovement(Message) (Variables|Default|GetmpTargetActor)))
      (Variables|Default|SetTargetMovement _returnvalue))
    (:then_1
      (bind _returnvalue_2 (Class|ArenaUnitInterface|GetAnimationManager(Message) (Variables|Default|GetmpTargetActor)))
      (Variables|Default|SetTargetSkeletalMesh (Class|AnimationManager|GetSkeletalMeshComponent _returnvalue_2)))))

(event EventActivateInner
  (params (stage :type Integer))
  (bind _targetskeletalmesh (Variables|Default|GetTargetSkeletalMesh))
  (Class|TiledMovement|SetStunned (Variables|Default|GetTargetMovement) true)
  (Utilities|IsValid _targetskeletalmesh
    (:Is%20Valid
      (bind _returnvalue (Niagara|SpawnSystemAttached "/Game/FX/Stun/NGR_SYS_Stun.NGR_SYS_Stun" _targetskeletalmesh (Variables|Default|GetAttachmentSocket) "0, 0, 0" "0, 0, 0" "SnapToTargetIncludingScale" true))
      (Variables|Default|SetSpawnedParticles _returnvalue))))

(event EventDeactivateInner
  (bind _spawnedparticles (Variables|Default|GetSpawnedParticles))
  (Class|TiledMovement|SetStunned (Variables|Default|GetTargetMovement) false)
  (Utilities|IsValid _spawnedparticles
    (:Is%20Valid
      (Components|DestroyComponent _spawnedparticles))))

(fn ConstructionScript)

(fn ReactivateInner
  (params (duration :type Integer) (stage :type Integer))
  (return (+ duration (Class|StatusEffect|GetDuration)) (Variables|Default|GetmStage)))