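; Infection status effect for arena actors that damages its target each time it is applied and shows smoke while active.
; Setup caches the target's damageable and tiled-movement interfaces through getter messages, though only the damageable is used here.
; Each apply sends a Damage task with the effect as initiator, while activation and deactivation toggle the InfectionSmoke component.
; Reactivation adds the new duration to the existing one and keeps the current stage.
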(event EventDeactivateInner
  (Components|Activation|Deactivate (Variables|Default|GetInfectionSmoke)))

(event EventActivateInner
  (params (stage :type Integer))
  (Components|Activation|Activate (Variables|Default|GetInfectionSmoke) true))

(event EventApplyInner
  (Class|Damageable|ExecuteDamageableTask (Variables|Default|GetTargetDamageable) (Utilities|Struct|MakeDamageableTask "Damage" (Variables|Default|GetDamage) self 0 0)))

(event EventSetupInner
  (bind _mptargetactor (Variables|Default|GetmpTargetActor))
  (bind _returnvalue (Class|ArenaUnitInterface|GetDamageable(Message) _mptargetactor))
  (Variables|Default|SetTargetDamageable _returnvalue)
  (bind _returnvalue_2 (Class|ArenaUnitInterface|GetTiledMovement(Message) _mptargetactor))
  (Variables|Default|SetTargetMovement _returnvalue_2))

(fn ConstructionScript)

(fn ReactivateInner
  (params (duration :type Integer) (stage :type Integer))
  (return (+ duration (Class|StatusEffect|GetDuration)) (Variables|Default|GetmStage)))