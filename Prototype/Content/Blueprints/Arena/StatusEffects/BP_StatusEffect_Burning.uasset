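; Burning status effect for the arena that deals damage to its target and shows burning particles while active.
; Setup caches the target's damageable and status effects manager through messages on the target actor.
; Each apply damages the target and deactivates any Hive effect on it.
; Reactivation adds the new duration to the current one and keeps the existing stage.
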(event EventSetupInner
  (bind _returnvalue (Class|ArenaUnitInterface|GetDamageable(Message) (Variables|Default|GetmpTargetActor)))
  (Variables|Default|SetTargetDamageable _returnvalue)
  (bind _returnvalue_2 (Class|ArenaUnitInterface|GetStatusEffectsManager(Message) (Variables|Default|GetmpTargetActor)))
  (Variables|Default|SetTargetStatusEffectsManager _returnvalue_2))

(event EventActivateInner
  (params (stage :type Integer))
  (Components|Activation|Activate (Variables|Default|GetBurningParticles) true))

(event EventDeactivateInner
  (Components|Activation|Deactivate (Variables|Default|GetBurningParticles)))

(event EventApplyInner
  (params (timeOfApplication :type ETimeOfApplication%20Enum :default "BeforeActions"))
  (Class|Damageable|Damage (Variables|Default|GetTargetDamageable) (Variables|Default|GetDamage))
  ;[0.7995 1 0] Burning always deactivates Hive effect.
  (Class|StatusEffectsManager|DeactivateStatusEffect (Variables|Default|GetTargetStatusEffectsManager) "/Game/Blueprints/Arena/StatusEffects/BP_StatusEffect_Hive.BP_StatusEffect_Hive_C"))

(fn ConstructionScript
  (|CallParentFunction))

(fn ReactivateInner
  (params (duration :type Integer) (stage :type Integer))
  (return (+ duration (Class|StatusEffect|GetDuration)) (Variables|Default|GetmStage)))