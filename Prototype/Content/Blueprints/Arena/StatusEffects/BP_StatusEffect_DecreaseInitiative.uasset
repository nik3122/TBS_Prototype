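; Arena status effect that lowers the target's initiative by applying a penalty to its reaction rate bonus.
; Setup caches the target's action manager; activation subtracts a floored fraction of the nominal reaction rate from the bonus.
; The subtracted amount is stored so deactivation adds back exactly that value.
; Reactivation adds the incoming duration to the effect's duration and keeps its own stage, ignoring the incoming one.
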(event EventActivateInner
  (params (stage :type Integer))
  (bind _targetactionmanager (Variables|Default|GetTargetActionManager))
  (Variables|Default|SetChangedReaction (Math|Float|Floor (* (Class|ActionManager|GetNominalReactionRate _targetactionmanager) (Variables|Default|GetReactionChange_S1))))
  (Class|ActionManager|SetReactionRateBonus _targetactionmanager (- (Class|ActionManager|GetReactionRateBonus _targetactionmanager) (Variables|Default|GetChangedReaction))))

(event EventSetupInner
  (bind _returnvalue (Class|ArenaUnitInterface|GetActionManager(Message) (Variables|Default|GetmpTargetActor)))
  (Variables|Default|SetTargetActionManager _returnvalue))

(event EventDeactivateInner
  (bind _targetactionmanager (Variables|Default|GetTargetActionManager))
  (Class|ActionManager|SetReactionRateBonus _targetactionmanager (+ (Class|ActionManager|GetReactionRateBonus _targetactionmanager) (Variables|Default|GetChangedReaction))))

(fn ConstructionScript)

(fn ReactivateInner
  (params (duration :type Integer) (stage :type Integer))
  (return (+ duration (Class|StatusEffect|GetDuration)) (Variables|Default|GetmStage)))