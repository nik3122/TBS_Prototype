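; Arena status effect for bleeding that deals damage to its target actor each time the effect is applied.
; Setup caches the target's damageable interface, and the apply step sends the Damage value through it.
; Activation and deactivation add no behavior.
; Reactivation adds the incoming duration to the value from GetDuration and keeps the current stage, ignoring the incoming one.
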(event EventSetupInner
  (bind _returnvalue (Class|ArenaUnitInterface|GetDamageable(Message) (Variables|Default|GetmpTargetActor)))
  (Variables|Default|SetTargetDamageable _returnvalue))

(event EventDeactivateInner)

(event EventActivateInner
  (params (stage :type Integer)))

(event EventApplyInner
  (Class|Damageable|Damage (Variables|Default|GetTargetDamageable) (Variables|Default|GetDamage)))

(fn ConstructionScript)

(fn ReactivateInner
  (params (duration :type Integer) (stage :type Integer))
  (return (+ duration (Class|StatusEffect|GetDuration)) (Variables|Default|GetmStage)))