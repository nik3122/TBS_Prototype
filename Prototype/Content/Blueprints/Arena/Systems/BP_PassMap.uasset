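; BP_PassMap is the arena's tile-grid map, drawing tile highlights and tracking whether the cursor is over it.
; InitTileGrid adds an instanced mesh for each valid tile free in the fire slot and sizes the cursor-overlap plane to the grid.
; A separate marker shows action placement.
; Helpers reuse instances by zero-scaling extras, but setup and distribution show/hide are disabled with FIX IT prints, and grid-tile show/hide is stubbed.
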(event OnBeginCursorOver(CursorOverlapPlane)
  (params (TouchedComponent :type Primitive%20Component%20Object%20Reference))
  (Variables|Default|SetIsCursorOver true))

(event OnEndCursorOver(CursorOverlapPlane)
  (params (TouchedComponent :type Primitive%20Component%20Object%20Reference))
  (Variables|Default|SetIsCursorOver false))

(event EventInitTileGrid
  (bind _returnvalue (Class|PassMap|GetTileRadius))
  (bind _returnvalue_2 (Class|PassMap|GetTileRadius))
  (bind _returnvalue_3 (/ _returnvalue 1e+02))
  (Variables|Default|SetFreeTileScale (Math|Vector|MakeVector _returnvalue_3 _returnvalue_3 _returnvalue_3))
  (Utilities|FlowControl|Sequence
    (:then_0
      (Components|InstancedStaticMesh|ClearInstances (Variables|Default|GetAvailableSetupTilesInstances))
      (for _index (range 0 (- (Class|PassMap|GetTilesNumber) 1))
        (if (Class|PassMap|IsTileValid (Class|PassMap|CoordfromIndex _index))
          (if (Class|PassMap|IsTileFreeatSlot (Class|PassMap|CoordfromIndex _index) "OccupationSlot_Fire")
            (Components|InstancedStaticMesh|AddInstance (Variables|Default|GetAvailableSetupTilesInstances) (Math|Transform|MakeTransform (Class|PassMap|GetTilePositionLocal (Class|PassMap|CoordfromIndex _index)) "0, 0, 0" "1,1,1"))))))
    (:then_1
      ;[1 1 1] Scale cursor overlap plane:
      (Transformation|SetRelativeScale3D (Variables|Default|GetCursorOverlapPlane) (Math|Vector|MakeVector (* (+ (Math|Conversions|ToFloat(Integer) (Class|PassMap|GetHeight)) 0.5) 0.0174 _returnvalue_2) (* _returnvalue_2 0.015 (+ (Math|Conversions|ToFloat(Integer) (Class|PassMap|GetWidth)) 0.5)) 1.0)))))

(event EventTick
  (params (DeltaSeconds :type Float%20%28single-precision%29)))

(fn ConstructionScript
  (bind _returnvalue (Class|PassMap|GetTileRadius))
  (bind _returnvalue_2 (/ _returnvalue 1e+02))
  (Utilities|FlowControl|Sequence
    (:then_0
      ;[1 1 1] Setting up new scale factor for tiles.
      (Variables|Default|SetFreeTileScale (Math|Vector|MakeVector _returnvalue_2 _returnvalue_2 _returnvalue_2)))
    (:then_1
      ;[1 1 1] Scaling selection tile mask.
      (Transformation|SetRelativeScale3D (Variables|Default|GetTileUnderCursor) (Variables|Default|GetFreeTileScale)))))

(fn ShowActionPlacementTile
  (params (ActionPlacement :type Int%20Point%20Structure))
  (if (Class|PassMap|IsTileValid ActionPlacement)
    (Transformation|SetRelativeLocation (Variables|Default|GetActionSetupPlacementTile) (+ "0, 0,10.000000" (Class|PassMap|GetTilePositionLocal ActionPlacement)) false false)
    (Rendering|SetVisibility (Variables|Default|GetActionSetupPlacementTile) true true)
    (else
      (Public|HideActionPlacementTile))))

(fn HideActionPlacementTile
  (Rendering|SetVisibility (Variables|Default|GetActionSetupPlacementTile) false true))

(fn ShowDistributionTiles
  (params (DistributionTiles :type Array%20of%20Int%20Point%20Structures))
  (Development|PrintString "FIX IT: temporary don't show any distribution tiles." false))

(fn ShowTilesInstances
  (params (TilesToShow :type Array%20of%20Int%20Point%20Structures) (InstancedTileMeshes :type Instanced%20Static%20Mesh%20Component%20Object%20Reference%20%28by%20ref%29))
  (bind _output_get (LocalVariables|SetLTilesLastIndex (Utilities|Array|LastIndex TilesToShow)))
  (if (>= _output_get 0)
    (Rendering|SetVisibility InstancedTileMeshes true false)
    (LocalVariables|SetLMeshesLastIndex (- (Components|InstancedStaticMesh|GetInstanceCount InstancedTileMeshes) 1))
    (Utilities|CreateMoreInstances InstancedTileMeshes (- (LocalVariables|GetLTilesLastIndex) (LocalVariables|GetLMeshesLastIndex))
      (:Out
        (LocalVariables|SetLMeshesLastIndex (- (Components|InstancedStaticMesh|GetInstanceCount InstancedTileMeshes) 1))
        (Utilities|FlowControl|Sequence
          (:then_0
            (for _index (range 0 (Math|Integer|Min(Integer) (LocalVariables|GetLTilesLastIndex) (LocalVariables|GetLMeshesLastIndex)))
              (Components|InstancedStaticMesh|UpdateInstanceTransform InstancedTileMeshes _index (Math|Transform|MakeTransform (Class|PassMap|GetTilePositionLocal (Utilities|Array|Get(acopy) TilesToShow _index)) "0, 0, 0" "1,1,1") false false false)))
          (:then_1
            (for _index_2 (range (+ (Math|Integer|Min(Integer) (LocalVariables|GetLTilesLastIndex) (LocalVariables|GetLMeshesLastIndex)) 1) (Math|Integer|Max(Integer) (LocalVariables|GetLTilesLastIndex) (LocalVariables|GetLMeshesLastIndex)))
              (Components|InstancedStaticMesh|UpdateInstanceTransform InstancedTileMeshes _index_2 (Math|Transform|MakeTransform "0, 0, 0" "0, 0, 0" "0.000000,0.000000,0.000000") false false false)))
          (:then_2
            (Utilities|MarkInstancesDirty InstancedTileMeshes)))))
    (else
      (Rendering|SetVisibility InstancedTileMeshes false false))))

(fn HideTileInstances
  (params (InstancedTileMeshes :type Instanced%20Static%20Mesh%20Component%20Object%20Reference%20%28by%20ref%29))
  (bind _returnvalue (Components|InstancedStaticMesh|GetInstanceCount InstancedTileMeshes))
  (bind _returnvalue_2 (- _returnvalue 1))
  (for _index (range 0 _returnvalue_2)
    (Components|InstancedStaticMesh|UpdateInstanceTransform InstancedTileMeshes _index (Math|Transform|MakeTransform "0, 0, 0" "0, 0, 0" "0.000000,0.000000,0.000000") false (== _index _returnvalue_2) false)))

(fn HideSetupTiles
  (Development|PrintString "FIX IT: temporary don't hide any setup tiles." false))

(fn HideDistributionTiles
  (Development|PrintString "FIX IT: temporary don't hide any distribution tiles." false))

(fn ShowGridTiles
  (params (Tiles :type Array%20of%20Int%20Point%20Structures)))

(fn HideGridTiles
  (params (Tiles :type Array%20of%20Int%20Point%20Structures)))

(fn ShowSetupTiles
  (params (PotentialSetupTiles :type Array%20of%20Int%20Point%20Structures) (AvailableSetupTiles :type Array%20of%20Int%20Point%20Structures))
  (Development|PrintString "FIX IT: temporary don't show any setup tiles." false))

(fn IsCursorOverPassMap
  (return (Variables|Default|GetIsCursorOver)))