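; BP_ActionViz previews an action's tile distribution in the arena by spawning a visualizer actor on its tiles.
; Show clears the previous preview, optionally skips the executor's tile, and faces each visualizer toward the next tile, with the last keeping the previous rotation.
; GetVizFromActionBehavior picks the class from behavior bitmask flags in fixed priority, such as footprint, defence, melee or heal.
; Hide destroys all tracked visualizers.
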(event EventBeginPlay)

(event EventTick
  (params (DeltaSeconds :type Float%20%28single-precision%29)))

(fn Show
  (params (ActionDistribution :type Array%20of%20Action%20Distribution%20Tile%20Structures) (ExcludeExecutorTile :type Boolean))
  (CallFunction|Hide)
  (for _index (range (select ExcludeExecutorTile 1 0) (Utilities|Array|LastIndex ActionDistribution))
    (Utilities|FlowControl|Sequence
      (:then_0
        (if (>= (Utilities|Array|LastIndex ActionDistribution) (+ _index 1))
          (LocalVariables|SetLRotator (Math|Conversions|RotationFromXVector (- (Class|PassMap|GetTilePositionWorld (Class|ArenaUtilities|GetPassMap) (.mtile (Utilities|Array|Get(acopy) ActionDistribution (+ _index 1)))) (Class|PassMap|GetTilePositionWorld (Class|ArenaUtilities|GetPassMap) (.mtile (Utilities|Array|Get(acopy) ActionDistribution _index))))))))
      (:then_1
        (if (Utilities|IsValidClass (CallFunction|GetVizfromActionBehavior (.mentrybehavior (Utilities|Array|Get(acopy) ActionDistribution _index))))
          (bind _returnvalue (Game|SpawnActorfromClass (CallFunction|GetVizfromActionBehavior (.mentrybehavior (Utilities|Array|Get(acopy) ActionDistribution _index))) (Math|Transform|MakeTransform (Class|PassMap|GetTilePositionWorld (Class|ArenaUtilities|GetPassMap) (.mtile (Utilities|Array|Get(acopy) ActionDistribution _index))) (LocalVariables|GetLRotator) "1,1,1") "AlwaysSpawn" 0 0))
          (Utilities|Array|Add (Variables|Default|GetSpawnedVisualizers) _returnvalue))))))

(fn Hide
  (for _array_element (Variables|Default|GetSpawnedVisualizers)
    (Actor|DestroyActor _array_element))
  (Utilities|Array|Clear (Variables|Default|GetSpawnedVisualizers)))

(fn GetVizfromActionBehavior
  (params (ActionBehavior :type Integer))
  (if (Math|Conversions|ToBoolean(Integer) (Class|KismetMathLibrary|AndIntInt ActionBehavior (|BitmaskLiteral 4)))
    (return "/Game/Blueprints/Arena/ActionViz/BP_ActionViz_Footprint.BP_ActionViz_Footprint_C")
    (elif (Math|Conversions|ToBoolean(Integer) (Class|KismetMathLibrary|AndIntInt ActionBehavior (|BitmaskLiteral 1024)))
      (if (Math|Conversions|ToBoolean(Integer) (Class|KismetMathLibrary|AndIntInt ActionBehavior (|BitmaskLiteral 8)))
        (return "/Game/Blueprints/Arena/ActionViz/BP_ActionViz_Defence.BP_ActionViz_Defence_C")
        (else
          (return "/Game/Blueprints/Arena/ActionViz/BP_ActionViz_Defence.BP_ActionViz_Defence_C")))
      (elif (Math|Conversions|ToBoolean(Integer) (Class|KismetMathLibrary|AndIntInt ActionBehavior (|BitmaskLiteral 8)))
        (return "/Game/Blueprints/Arena/ActionViz/BP_ActionViz_MeleeAttack.BP_ActionViz_MeleeAttack_C")
        (elif (Math|Conversions|ToBoolean(Integer) (Class|KismetMathLibrary|AndIntInt ActionBehavior (|BitmaskLiteral 16)))
          (return "/Game/Blueprints/Arena/ActionViz/BP_ActionViz_Heal.BP_ActionViz_Heal_C")
          (elif (Math|Conversions|ToBoolean(Integer) (Class|KismetMathLibrary|AndIntInt ActionBehavior (|BitmaskLiteral 128)))
            (return "/Game/Blueprints/Arena/ActionViz/BP_ActionViz_Summon.BP_ActionViz_Summon_C")
            (elif (Math|Conversions|ToBoolean(Integer) (Class|KismetMathLibrary|AndIntInt ActionBehavior (|BitmaskLiteral 256)))
              (return "/Game/Blueprints/Arena/ActionViz/BP_ActionViz_Trap.BP_ActionViz_Trap_C")
              (elif (Math|Conversions|ToBoolean(Integer) (Class|KismetMathLibrary|AndIntInt ActionBehavior (|BitmaskLiteral 512)))
                (return "/Game/Blueprints/Arena/ActionViz/BP_ActionViz_Mental.BP_ActionViz_Mental_C")
                (elif (Math|Conversions|ToBoolean(Integer) (Class|KismetMathLibrary|AndIntInt ActionBehavior (|BitmaskLiteral 32)))
                  (return "/Game/Blueprints/Arena/ActionViz/BP_ActionViz_Buff.BP_ActionViz_Buff_C")
                  (elif (Math|Conversions|ToBoolean(Integer) (Class|KismetMathLibrary|AndIntInt ActionBehavior (|BitmaskLiteral 64)))
                    (return "/Game/Blueprints/Arena/ActionViz/BP_ActionViz_Debuff.BP_ActionViz_Debuff_C")
                    (else
                      (return 0))))))))))))