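; BP_HiveBox is a destructible arena unit that spreads the Hive status effect when it dies.
; On death it gathers both player and AI party members, sorts them by pass-map distance from its tile, and infects the first NumberOfTargetsToInfect with an effectively permanent effect.
; For each target it spawns a BP_HiveVisual at the box and binds it to that effect, then destroys itself.
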(event MEventDeath(Damageable)
  (CallFunction|ActivateStatusEffects)
  (Actor|DestroyActor))

(fn ConstructionScript
  (|CallParentFunction))

(fn ActivateStatusEffects
  (bind _arenamanagerinterface (Utilities|GetArenaManager))
  (Utilities|FlowControl|Sequence
    (:then_0
      (bind _returnvalue (Class|ArenaManagerInterface|GetPlayerParty _arenamanagerinterface))
      (Utilities|Array|AppendArray (LocalVariables|GetLTargetCreatures) (Class|Party|GetMembers _returnvalue))
      (bind _returnvalue_2 (Class|ArenaManagerInterface|GetAIParty _arenamanagerinterface))
      (Utilities|Array|AppendArray (LocalVariables|GetLTargetCreatures) (Class|Party|GetMembers _returnvalue_2)))
    (:then_1
      (Class|PassMap|SortCreaturesbyDistancetoTile (Utilities|GetPassMap) (LocalVariables|GetLTargetCreatures) (Class|TiledMovement|GetCurrentTile (Variables|Default|GetTiledMovement)) (LocalVariables|GetLDistancesToTargets)))
    (:then_2
      (for _index (range 0 (- (Variables|Default|GetNumberOfTargetsToInfect) 1))
        (Class|StatusEffectsManager|ActivateStatusEffect (Class|CreatureBase|GetStatusEffectsManagerComponent (Utilities|Array|Get(acopy) (LocalVariables|GetLTargetCreatures) _index)) "/Game/Blueprints/Arena/StatusEffects/BP_StatusEffect_Hive.BP_StatusEffect_Hive_C" 99999 (Variables|Default|GetHiveEffectStage) 99999)
        (bind _returnvalue_3 (Game|SpawnActorfromClass "/Game/Blueprints/Arena/BP_HiveVisual.BP_HiveVisual_C" (Math|Transform|MakeTransform (Transformation|GetActorLocation) "0, 0, 0" "1,1,1") "Undefined" 0 0))
        (bind _asbp_status_effect_hive (Utilities|Casting|CastToBP_StatusEffect_Hive (Class|StatusEffectsManager|GetEffectbyType (Class|CreatureBase|GetStatusEffectsManagerComponent (Utilities|Array|Get(acopy) (LocalVariables|GetLTargetCreatures) _index)) "/Game/Blueprints/Arena/StatusEffects/BP_StatusEffect_Hive.BP_StatusEffect_Hive_C")))
        (Default|BindHiveVisual _asbp_status_effect_hive _returnvalue_3)))))

(fn GetActionManager
  (return 0))

(fn GetAnimationManager
  (return 0))

(fn GetDamageable
  (return (Variables|Default|GetDamageable)))

(fn GetSocialComponent
  (return 0))

(fn GetStatusEffectsManager
  (return 0))

(fn GetTiledMovement
  (return (Variables|Default|GetTiledMovement)))

(fn GetWeaponOperator
  (return 0))