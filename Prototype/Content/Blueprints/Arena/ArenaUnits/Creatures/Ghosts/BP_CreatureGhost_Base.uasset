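; Base Blueprint for arena creature ghosts, tinting the skeletal mesh in the party member color of its associated creature.
; The construction script creates a dynamic MAT_Ghost instance on the first material slot and stores it as GhostMaterial.
; It sets both BaseColor and CounterColor to that color at half brightness, with alpha pushed above one.
; The event graph holds only disabled placeholder events.
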(event EventBeginPlay)

(event Collision|EventActorBeginOverlap
  (params (OtherActor :type Actor%20Object%20Reference)))

(event EventTick
  (params (DeltaSeconds :type Float%20%28single-precision%29)))

(fn ConstructionScript
  (bind _massociatedcreature (Variables|Default|GetmAssociatedCreature))
  (bind _returnvalue (Class|CreatureBase|GetPartyMemberColor _massociatedcreature))
  (bind _returnvalue_2 (* (.b _returnvalue) 0.5))
  (bind _returnvalue_3 (* (.r _returnvalue) 0.5))
  (bind _returnvalue_4 (* (.g _returnvalue) 0.5))
  (bind _returnvalue_5 (Math|Color|MakeColor _returnvalue_3 _returnvalue_4 _returnvalue_2 4.0))
  (bind _returnvalue_6 (Rendering|Material|CreateDynamicMaterialInstance (Variables|Default|GetSkeletalMesh) 0 "/Game/Materials/MAT_Ghost.MAT_Ghost" "None" :!class /Script/Engine.PrimitiveComponent))
  (bind _output_get (Variables|Default|SetGhostMaterial _returnvalue_6))
  (Rendering|Material|SetMaterial (Variables|Default|GetSkeletalMesh) 0 _output_get)
  (Rendering|Material|SetVectorParameterValue (Variables|Default|GetGhostMaterial) "BaseColor" _returnvalue_5 :!class /Script/Engine.MaterialInstanceDynamic)
  (Rendering|Material|SetVectorParameterValue (Variables|Default|GetGhostMaterial) "CounterColor" _returnvalue_5 :!class /Script/Engine.MaterialInstanceDynamic))