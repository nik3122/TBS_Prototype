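; Base Blueprint for creature units in the arena, showing each on a platform tinted with its party member color.
; On BeginPlay it creates a dynamic material for the platform and sets the color parameter, updating it whenever the party member color changes.
; It exposes getters for picture, name and tooltip description, leaves the head position getter empty, and forwards focus state to the HP change visualizer.
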(event EventBeginPlay
  (bind _returnvalue (Rendering|Material|CreateDynamicMaterialInstance (Variables|Default|GetPlatform) 0 "/Game/FX/CharacterPlatform/MAT_CharacterPlatform.MAT_CharacterPlatform" "None" :!class /Script/Engine.PrimitiveComponent))
  (bind _output_get (Variables|Default|SetPlatformMaterial _returnvalue))
  (Rendering|Material|SetMaterial (Variables|Default|GetPlatform) 0 _output_get)
  (Rendering|Material|SetVectorParameterValue (Variables|Default|GetPlatformMaterial) "PartyMemberColor" (Class|CreatureBase|GetPartyMemberColor) :!class /Script/Engine.MaterialInstanceDynamic))

(event EventOnPartyMemberColorChanged
  (Rendering|Material|SetVectorParameterValue (Variables|Default|GetPlatformMaterial) "PartyMemberColor" (Class|CreatureBase|GetPartyMemberColor) :!class /Script/Engine.MaterialInstanceDynamic))

(fn ConstructionScript)

(fn GetCreaturePicture
  (return (Variables|Unknown|GetCreaturePicture)))

(fn GetCreatureName
  (return (Variables|Unknown|GetCreatureName)))

(fn GetCreatureDescriptionToolTip
  (return (Variables|Unknown|GetCreatureDescriptionToolTip)))

(fn GetHeadPosition)

(fn SetIsFocused
  (params (IsFocused :type Boolean))
  (Default|SetIsFocused (Variables|Default|GetBP_HPChangeVisualizer) IsFocused))