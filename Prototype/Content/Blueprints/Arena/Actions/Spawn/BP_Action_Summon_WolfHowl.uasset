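; Arena summon action for a wolf howl that allows a spawn only when enough howls collide on one tile.
; Colliding howls share a CollisionStack without interrupting each other, and only the action at the limit position sets MIsSpawnAllowed; other collisions defer to the parent.
; It exploits collision resolution to update that flag just in time, assuming single-tile collisions.
; Setup visualization shows the action distribution, excluding the executor's tile.
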(event EventStartSetupVisualization
  (if (Class|ActionBase|IsSetup)
    (Default|Show (Variables|Default|GetActionViz) (Variables|Default|GetmDistribution) true)))

(event EventStopSetupVisualization
  (Default|Hide (Variables|Default|GetActionViz)))

(event EventReset
  (bind _collisionstack (Variables|Default|GetCollisionStack))
  (|CallParentFunction)
  (Utilities|Array|Clear _collisionstack)
  (Utilities|Array|Add _collisionstack self)
  (Variables|Default|SetmIsSpawnAllowed false))

(event EventOnFinishCollisionResolve
  (CallFunction|UpdateIsSpawnAllowed)
  (if (Variables|Default|GetmIsSpawnAllowed)
    (Development|PrintString (Utilities|String|Append (Utilities|GetObjectName (Class|ActionBase|GetExecutorActor)) "->" (Utilities|GetObjectName self) " spawn allowed.") false true "(R=0.000000,G=0.397106,B=1.000000,A=1.000000)" 5.0)))

(fn ConstructionScript
  (|CallParentFunction))

(fn ResolveCollision
  (params (pLowPriorityAction :type Action%20Base%20Object%20Reference) (collisionPlacement :type Int%20Point%20Structure%20%28by%20ref%29) (highPrioEntryBehavior :type Integer) (lowPrioEntryBehavior :type Integer))
  ;[1 0.7578 0] HACK: ResolveCollision is called when action wasn't interrupted / cancelled. Thus we can exploit it to set mIsSpawnAllowed "just in time".
  (Utilities|EXPLOITACTIONRESOLVE
    (:Out
      (CallFunction|UpdateIsSpawnAllowed)
      (bind _asbp_action_summon_wolf_howl (Utilities|Casting|CastToBP_Action_Summon_WolfHowl pLowPriorityAction)
        (:then
          ;[1 0.0124 0] Assume a collision takes place only in a single tile. Otherwise collisions in other tiles would be counted into single collision stack.
          (Utilities|Array|AddUnique (Variables|Default|GetCollisionStack) _asbp_action_summon_wolf_howl)
          (Utilities|Array|Clear (Variables|BP_Action_Summon_WolfHowl_C|GetCollisionStack _asbp_action_summon_wolf_howl))
          (Utilities|Array|AppendArray (Variables|BP_Action_Summon_WolfHowl_C|GetCollisionStack _asbp_action_summon_wolf_howl) (Variables|Default|GetCollisionStack))
          (return (Utilities|Struct|MakeActionCollisionResolveResult false 0)))
        (:CastFailed
          (bind _returnvalue (|CallParentFunction pLowPriorityAction collisionPlacement highPrioEntryBehavior lowPrioEntryBehavior))
          (return _returnvalue))))))

(fn UpdateIsSpawnAllowed
  (bind _self self)
  (bind _collisionstacklimit (Variables|Default|GetCollisionStackLimit))
  (bind _returnvalue (- _collisionstacklimit 1))
  (if (Utilities|Array|IsValidIndex (Variables|Default|GetCollisionStack) _returnvalue)
    (Variables|/Script/Prototype.Action_Spawn_Base|SetmIsSpawnAllowed _self (== _self (Utilities|Array|Get(acopy) (Variables|Default|GetCollisionStack) _returnvalue)))))