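; Base arena action that places a trap of a configurable type on its placement tile through the trap system.
; Execution plays the executor's montage and spawns on its notify, with post-execution as fallback and a flag preventing double spawns.
; Setup and distribution require free tile occupation slots in the pass map.
; The action claims its tile, and collisions interrupt when both actions pretend on the collision tile.
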(event EventStopClaimingTile
  (params (tile :type Int%20Point%20Structure%20%28by%20ref%29)))

(event EventPreExecutionApply)

(event EventPostExecutionApply
  (if (not (Variables|Default|GetmIsCanceled))
    (CallFunction|SpawnTrap)))

(event EventOnStartExecution
  (if (not (Variables|Default|GetmIsCanceled))
    (bind _animationmanager (Utilities|IfExecutorHasAnimationManager)
      (:Is%20Valid
        (Animation|Montage|PlayMontage (Class|AnimationManager|GetSkeletalMeshComponent _animationmanager) (Class|AnimationManager|GetSingleActionsAnimMontage _animationmanager) 1.0 0.0 (Variables|Default|GetActionSectionName)
          (:OnCompleted
            (Class|ActionBase|StopExecution :!label _label))
          (:OnNotifyBegin
            (CallFunction|SpawnTrap))))
      (:Is%20Not%20Valid
        (goto _label)))))

(event EventOnStopExecution)

(event EventReset
  (|CallParentFunction)
  (Variables|Default|SetIsTrapSpawned false))

(fn ConstructionScript)

(fn IsPretendingonTile
  (params (tile :type Int%20Point%20Structure%20%28by%20ref%29))
  (return (Utilities|EqualTiles tile (Class|ActionBase|GetPlacement))))

(fn ResolveCollision
  (params (pLowPriorityAction :type Action%20Base%20Object%20Reference) (collisionPlacement :type Int%20Point%20Structure%20%28by%20ref%29) (highPrioEntryBehavior :type Integer) (lowPrioEntryBehavior :type Integer))
  (return (Utilities|Struct|MakeActionCollisionResolveResult (and (CallFunction|IsPretendingonTile pLowPriorityAction collisionPlacement) (CallFunction|IsPretendingonTile collisionPlacement)) true 0)))

(fn OnInterrupt
  (params (interruptionTile :type Int%20Point%20Structure%20%28by%20ref%29) (pInterrupterAction :type Action%20Base%20Object%20Reference))
  (return true))

(fn SpawnTrap
  (if (not (Variables|Default|GetIsTrapSpawned))
    (Variables|Default|SetIsTrapSpawned true)
    (Class|TrapSystem|TrySpawnTrap (Class|ArenaUtilities|GetTrapSystem) (Variables|Default|GetTrapType) (Class|ActionBase|GetPlacement))))

(fn TryDistributeat
  (params (potentialDistributionTile :type Int%20Point%20Structure%20%28by%20ref%29))
  (if (Class|PassMap|IsTileFree (Class|ArenaUtilities|GetPassMap) potentialDistributionTile (|BitmaskLiteral 7) false)
    (return (Variables|Default|GetmActionBehavior) true)
    (else
      (return 0 false))))

(fn CanbeSetupat
  (params (potentialSetupTile :type Int%20Point%20Structure%20%28by%20ref%29))
  (return (Class|PassMap|IsTileFree (Class|ArenaUtilities|GetPassMap) potentialSetupTile (|BitmaskLiteral 7) false)))

(fn FinalizeSetupProcess
  (return true))

(fn IsClaimingTile
  (params (tile :type Int%20Point%20Structure%20%28by%20ref%29))
  (return (Utilities|EqualTiles tile (Class|ActionBase|GetPlacement))))