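; Base Blueprint for arena summon actions, handling the tile visualization shown during action setup.
; When setup visualization starts and the action is set up, it shows its distribution through ActionViz, excluding the executor's tile.
; Stopping setup visualization hides it, and the tile-claiming check simply defers to the parent class.
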(event EventStartSetupVisualization
  (if (Class|ActionBase|IsSetup)
    (Default|Show (Variables|Default|GetActionViz) (Variables|Default|GetmDistribution) true)))

(event EventStopSetupVisualization
  (Default|Hide (Variables|Default|GetActionViz)))

(fn ConstructionScript)

(fn IsClaimingTile
  (params (tile :type Int%20Point%20Structure%20%28by%20ref%29))
  (return (|CallParentFunction tile)))