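; Arena action Mind Blur, which cancels a colliding lower-priority action of another unit and plays a blur effect on that unit.
; Setup and distribution accept only tiles occupied by arena units with an action manager.
; ResolveCollision checks a behavior bit, stores that action's executor as Target and returns a huge cancellation count.
; Execution, unless canceled, attaches particles to the Target's head and plays the executor's action animation, stopping if it cannot play.
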(event EventReset
  (|CallParentFunction)
  (Variables|Default|SetTarget 0))

(event EventPreExecutionApply)

(event EventPostExecutionApply)

(event EventOnStopExecution
  (bind _animationmanager (Utilities|IfExecutorHasAnimationManager)
    (:Is%20Valid
      (EventDispatchers|UnbindEventfromMEventSingleActionAnimationFinished _animationmanager (EventDispatchers|CreateEvent :!event StopExecution)))))

(event EventOnStartExecution
  (bind _target (Variables|Default|GetTarget))
  (bind _returnvalue (Actor|GetComponentbyClass _target "/Script/Engine.SkeletalMeshComponent"))
  (if (not (Variables|Default|GetmIsCanceled))
    (Utilities|FlowControl|Sequence
      (:then_0
        (Utilities|IsValid _target
          (:Is%20Valid
            (Utilities|IsValid _returnvalue
              (:Is%20Valid
                (Effects|SpawnEmitterAttached "/Game/FX/MindBlur/PART_MindBlur.PART_MindBlur" _returnvalue "Head" "0, 0, 0" "0, 0, 0" "1.000000,1.000000,1.000000" "SnapToTarget" true "AutoRelease"))))))
      (:then_1
        (bind _animationmanager (Utilities|IfExecutorHasAnimationManager)
          (:Is%20Valid
            (bind _returnvalue_2 (Class|AnimationManager|TryPlaySingleActionAnimation _animationmanager (Variables|Default|GetActionAnimationSection)))
            (if _returnvalue_2
              (EventDispatchers|BindEventtoMEventSingleActionAnimationFinished _animationmanager (EventDispatchers|CreateEvent :!event StopExecution))
              (else
                (Class|ActionBase|StopExecution :!label _label))))
          (:Is%20Not%20Valid
            (goto _label)))))))

(fn ConstructionScript)

(fn ResolveCollision
  (params (pLowPriorityAction :type Action%20Base%20Object%20Reference) (collisionPlacement :type Int%20Point%20Structure%20%28by%20ref%29) (highPrioEntryBehavior :type Integer) (lowPrioEntryBehavior :type Integer))
  (if (Math|Conversions|ToBoolean(Integer) (Class|KismetMathLibrary|AndIntInt lowPrioEntryBehavior (|BitmaskLiteral 2)))
    (Variables|Default|SetTarget (Class|ActionBase|GetExecutorActor pLowPriorityAction))
    (return (Utilities|Struct|MakeActionCollisionResolveResult false 999999))
    (else
      (return (Utilities|Struct|MakeActionCollisionResolveResult false 0)))))

(fn CanbeSetupat
  (params (potentialSetupTile :type Int%20Point%20Structure%20%28by%20ref%29))
  (bind _asarena_unit_interface (Utilities|Casting|CastToArenaUnit_Interface (Class|PassMap|GetOccupant (Class|ArenaUtilities|GetPassMap) potentialSetupTile "OccupationSlot_ArenaUnit"))
    (:then
      (bind _returnvalue (Class|ArenaUnitInterface|GetActionManager _asarena_unit_interface))
      (return (Utilities|IsValid _returnvalue)))
    (:CastFailed
      (return false))))

(fn TryDistributeat
  (params (potentialDistributionTile :type Int%20Point%20Structure%20%28by%20ref%29))
  (bind _asarena_unit_interface (Utilities|Casting|CastToArenaUnit_Interface (Class|PassMap|GetOccupant (Class|ArenaUtilities|GetPassMap) potentialDistributionTile "OccupationSlot_ArenaUnit"))
    (:then
      (bind _returnvalue (Class|ArenaUnitInterface|GetActionManager _asarena_unit_interface))
      (return (Variables|Default|GetmActionBehavior) (Utilities|IsValid _returnvalue)))
    (:CastFailed
      (return 0 false))))

(fn FinalizeSetupProcess
  (return true))