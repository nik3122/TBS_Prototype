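; Arena action that heals creatures on its target tiles by a set HP amount.
; Setup and distribution accept only tiles whose arena-unit occupant is a creature, collecting its damageable component, and healing runs as a damageable task before execution apply.
; On start, the executor aims at the placement tile, spawns Niagara effects on targets and plays an animation, stopping immediately if none can play.
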(event EventReset
  (|CallParentFunction)
  (Utilities|Array|Clear (Variables|Default|GetTargetDamageables)))

(event EventPreExecutionApply
  (for _array_element (Variables|Default|GetTargetDamageables)
    (Class|Damageable|ExecuteDamageableTask _array_element (Utilities|Struct|MakeDamageableTask "Heal" (Utilities|Struct|MakeDamageParameters (Variables|Default|GetHealHPAmount) 0 0 0 0) (Class|ActionBase|GetExecutorActor) (Class|ActionBase|GetExecutionPriority) 0))))

(event EventPostExecutionApply)

(event EventOnStopExecution
  (bind _animationmanager (Utilities|IfExecutorHasAnimationManager)
    (:Is%20Valid
      (EventDispatchers|UnbindEventfromMEventSingleActionAnimationFinished _animationmanager (EventDispatchers|CreateEvent :!event StopExecution)))))

(event EventOnStartExecution
  (Class|TiledMovement|AimatTile (Class|ActionBase|GetExecutorTiledMovement) (Class|ActionBase|GetPlacement))
  (if (not (Variables|Default|GetmIsCanceled))
    (Utilities|FlowControl|Sequence
      (:then_0
        (for _array_element (Variables|Default|GetTargetDamageables)
          (Niagara|SpawnSystematLocation "/Game/FX/Heal/NGR_SYS_HealNeighbor.NGR_SYS_HealNeighbor" (Transformation|GetActorLocation (Components|GetOwner _array_element)))))
      (:then_1
        (bind _animationmanager (Utilities|IfExecutorHasAnimationManager)
          (:Is%20Valid
            (bind _returnvalue (Class|AnimationManager|TryPlaySingleActionAnimation _animationmanager (Variables|Default|GetActionSectionName)))
            (if _returnvalue
              (EventDispatchers|BindEventtoMEventSingleActionAnimationFinished _animationmanager (EventDispatchers|CreateEvent :!event StopExecution))
              (else
                (Class|ActionBase|StopExecution))))
          (:Is%20Not%20Valid
            (Class|ActionBase|StopExecution)))))))

(fn ConstructionScript)

(fn ResolveCollision
  (params (pLowPriorityAction :type Action%20Base%20Object%20Reference) (collisionPlacement :type Int%20Point%20Structure%20%28by%20ref%29) (highPrioEntryBehavior :type Integer) (lowPrioEntryBehavior :type Integer))
  (return (Utilities|Struct|MakeActionCollisionResolveResult false 0)))

(fn CanbeSetupat
  (params (potentialSetupTile :type Int%20Point%20Structure%20%28by%20ref%29))
  (return (.bSuccess (Utilities|Casting|CastToCreatureBase (Class|PassMap|GetOccupant (Class|ArenaUtilities|GetPassMap) potentialSetupTile "OccupationSlot_ArenaUnit")))))

(fn TryDistributeat
  (params (potentialDistributionTile :type Int%20Point%20Structure%20%28by%20ref%29))
  (bind _ascreature_base (Utilities|Casting|CastToCreatureBase (Class|PassMap|GetOccupant (Class|ArenaUtilities|GetPassMap) potentialDistributionTile "OccupationSlot_ArenaUnit"))
    (:then
      (Utilities|Array|Add (Variables|Default|GetTargetDamageables) (Class|CreatureBase|GetDamageableComponent _ascreature_base))
      (return (Variables|Default|GetmActionBehavior) true))
    (:CastFailed
      (return 0 false))))

(fn FinalizeSetupProcess
  (return true))