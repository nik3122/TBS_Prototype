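; Arena action, set up on creature-occupied tiles, that copies another unit's action for its executor.
; On collision, it stores the class and executor of a recordable lower-priority action with the required behavior flag, without interrupting it.
; Execution plays a single-action animation, stopping immediately if that fails.
; Unless canceled, post-execution grants the recorded class through the executor's action manager for limited turns.
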(event EventOnStopExecution
  (bind _animationmanager (Utilities|IfExecutorHasAnimationManager)
    (:Is%20Valid
      (EventDispatchers|UnbindEventfromMEventSingleActionAnimationFinished _animationmanager (EventDispatchers|CreateEvent :!event StopExecution)))))

(event EventOnCancel
  (params (pCancelerAction :type Action%20Base%20Object%20Reference))
  (Variables|Default|SetRecorderedActionClass 0))

(event EventReset
  (Variables|Default|SetRecorderedActionClass 0)
  (Variables|Default|SetTarget 0))

(event EventPreExecutionApply)

(event EventPostExecutionApply
  (if (not (Variables|Default|GetmIsCanceled))
    (if (Utilities|IsValidClass (Variables|Default|GetRecorderedActionClass))
      (bind _actionmanager (Utilities|IfExecutorHasActionManager)
        (:Is%20Valid
          (Class|ActionManager|AddAction _actionmanager (Variables|Default|GetRecorderedActionClass) (Variables|Default|GetActionAvailabilityDuration)))))))

(event EventOnStartExecution
  (if (not (Variables|Default|GetmIsCanceled))
    (bind _animationmanager (Utilities|IfExecutorHasAnimationManager)
      (:Is%20Valid
        (bind _returnvalue (Class|AnimationManager|TryPlaySingleActionAnimation _animationmanager (Variables|Default|GetAnimSectionName)))
        (if _returnvalue
          (EventDispatchers|BindEventtoMEventSingleActionAnimationFinished _animationmanager (EventDispatchers|CreateEvent :!event StopExecution))
          (else
            (Class|ActionBase|StopExecution :!label _label))))
      (:Is%20Not%20Valid
        (goto _label)))))

(fn ConstructionScript)

(fn ResolveCollision
  (params (pLowPriorityAction :type Action%20Base%20Object%20Reference) (collisionPlacement :type Int%20Point%20Structure%20%28by%20ref%29) (highPrioEntryBehavior :type Integer) (lowPrioEntryBehavior :type Integer))
  (if (and (Class|ActionBase|IsRecordable pLowPriorityAction) (Math|Conversions|ToBoolean(Integer) (Class|KismetMathLibrary|AndIntInt lowPrioEntryBehavior (|BitmaskLiteral 2))))
    (Variables|Default|SetRecorderedActionClass (Utilities|GetClass pLowPriorityAction))
    (Variables|Default|SetTarget (Class|ActionBase|GetExecutorActor pLowPriorityAction)))
  (return (Utilities|Struct|MakeActionCollisionResolveResult false 0)))

(fn CanbeSetupat
  (params (potentialSetupTile :type Int%20Point%20Structure%20%28by%20ref%29))
  (return (.bSuccess (Utilities|Casting|CastToCreatureBase (Class|PassMap|GetOccupantSafe (Class|ArenaUtilities|GetPassMap) potentialSetupTile "OccupationSlot_ArenaUnit")))))

(fn TryDistributeat
  (params (potentialDistributionTile :type Int%20Point%20Structure%20%28by%20ref%29))
  (return (Variables|Default|GetmActionBehavior) (.bSuccess (Utilities|Casting|CastToCreatureBase (Class|PassMap|GetOccupantSafe (Class|ArenaUtilities|GetPassMap) potentialDistributionTile "OccupationSlot_ArenaUnit")))))

(fn FinalizeSetupProcess
  (return true))