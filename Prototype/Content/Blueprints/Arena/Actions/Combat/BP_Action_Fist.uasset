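; BP_Action_Fist is an arena combat action whose collision resolution lets Fist actions stack.
; When it collides with a lower-priority Fist and neither entry behavior has bit 2 set, it increments that Fist's stack without interrupting.
; Otherwise, reaching its own stack threshold returns a huge cancellation counter change without interrupting, while smaller stacks defer to parent resolution.
; Reset clears the stack.
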(event EventReset
  (Variables|Default|SetCollisionStackSize 0)
  (|CallParentFunction))

(fn ConstructionScript
  (|CallParentFunction))

(fn ResolveCollision
  (params (pLowPriorityAction :type Action%20Base%20Object%20Reference) (collisionPlacement :type Int%20Point%20Structure%20%28by%20ref%29) (highPrioEntryBehavior :type Integer) (lowPrioEntryBehavior :type Integer))
  (bind _returnvalue (|BitmaskLiteral 2))
  (bind (_asbp_action_fist _bsuccess) (Utilities|Casting|CastToBP_Action_Fist pLowPriorityAction))
  (if (Math|Boolean|ANDBoolean _bsuccess (not (Math|Conversions|ToBoolean(Integer) (Class|KismetMathLibrary|AndIntInt _returnvalue highPrioEntryBehavior))) (not (Math|Conversions|ToBoolean(Integer) (Class|KismetMathLibrary|AndIntInt _returnvalue lowPrioEntryBehavior))))
    (Math|Integer|IncrementInt (Variables|BP_Action_Fist_C|GetCollisionStackSize _asbp_action_fist)
      (:%20%20
        (return (Utilities|Struct|MakeActionCollisionResolveResult false 0))))
    (elif (>= (Variables|Default|GetCollisionStackSize) (Variables|Default|GetCollisionStackSizeToSucceed))
      (return (Utilities|Struct|MakeActionCollisionResolveResult false 999999))
      (else
        (bind _returnvalue_2 (|CallParentFunction pLowPriorityAction collisionPlacement highPrioEntryBehavior lowPrioEntryBehavior))
        (return _returnvalue_2)))))