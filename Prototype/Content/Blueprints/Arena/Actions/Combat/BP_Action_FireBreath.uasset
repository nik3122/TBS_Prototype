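; BP_Action_FireBreath is an arena combat action that breathes fire and sets tiles alight.
; On execution start, unless canceled, it attaches a fire breath particle effect to the executor's skeletal mesh at the breath socket.
; It stops executing only once both animation and particles finish, using two flags cleared on reset.
; After applying, it ignites every distribution tile through the fire system; its TryDistributeAt override accepts any candidate tile.
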(event Custom|ParticlesFinished
  (params (PSystem :type Particle%20System%20Component%20Object%20Reference))
  (Variables|Default|SetIsParticlesFinished true)
  (if (Variables|Default|GetIsAnimationFinished)
    (Class|ActionBase|StopExecution)))

(event EventPostExecutionApply
  (|CallParentFunction)
  (for _array_element (Variables|Default|GetmDistribution)
    (Class|FireSystem|SetTileonFire (Class|ArenaUtilities|GetFireSystem) (.mtile _array_element))))

(event EventOnStartExecution
  (|CallParentFunction)
  (if (not (Variables|Default|GetmIsCanceled))
    (bind _animationmanager (Utilities|IfExecutorHasAnimationManager)
      (:Is%20Valid
        (bind _returnvalue (Effects|SpawnEmitterAttached "/Game/FX/FireBreath/PART_FireBreath.PART_FireBreath" (Class|AnimationManager|GetSkeletalMeshComponent _animationmanager) "FireBreathStartPoint" "0, 0, 0" "0, 0, 0" "1.000000,1.000000,1.000000" "SnapToTargetIncludingScale" true "AutoRelease"))
        (EventDispatchers|BindEventtoOnSystemFinished _returnvalue (EventDispatchers|CreateEvent :!event Custom|ParticlesFinished))))))

(event EventOnAnimationFinished
  (Variables|Default|SetIsAnimationFinished true)
  (if (Variables|Default|GetIsParticlesFinished)
    (Class|ActionBase|StopExecution)))

(event EventReset
  (|CallParentFunction)
  (Variables|Default|SetIsAnimationFinished false)
  (Variables|Default|SetIsParticlesFinished false))

(fn ConstructionScript
  (|CallParentFunction))

(fn TryDistributeat
  (params (potentialDistributionTile :type Int%20Point%20Structure%20%28by%20ref%29))
  (|CallParentFunction potentialDistributionTile)
  (return (Variables|Default|GetmActionBehavior) true))