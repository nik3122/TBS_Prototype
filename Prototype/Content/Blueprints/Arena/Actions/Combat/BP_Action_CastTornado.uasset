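; Combat action for the tile-based arena that casts a tornado along its distributed tiles and damages creatures caught in it.
; Collision resolution collects victims and decides whether to interrupt their lower-priority actions, based on placement, entry behavior and idleness.
; Before execution applies, each victim receives a prioritized damage task linked to a battle log item.
; Execution spawns BP_Tornado on the tile path and plays the caster's animation, stopping immediately if it cannot play.
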(event EventPreExecutionApply
  (CallFunction|AffectTargets))

(event EventOnStartExecution
  (if (not (Variables|Default|GetmIsCanceled))
    (CallFunction|StartTornado)
    (bind _animationmanager (Utilities|IfExecutorHasAnimationManager)
      (:Is%20Valid
        (bind _returnvalue (Class|AnimationManager|TryPlaySingleActionAnimation _animationmanager (Variables|Default|GetSingleAnimationSection)))
        (if _returnvalue
          (EventDispatchers|BindEventtoMEventSingleActionAnimationFinished _animationmanager (EventDispatchers|CreateEvent :!event StopExecution))
          (else
            (Class|ActionBase|StopExecution :!label _label))))
      (:Is%20Not%20Valid
        (goto _label)))))

(event EventPostExecutionApply)

(event EventOnStopExecution
  (bind _animationmanager (Utilities|IfExecutorHasAnimationManager)
    (:Is%20Valid
      (EventDispatchers|UnbindEventfromMEventSingleActionAnimationFinished _animationmanager (EventDispatchers|CreateEvent :!event StopExecution)))))

(fn ConstructionScript)

(fn IsPretendingonTile
  (params (tile :type Int%20Point%20Structure%20%28by%20ref%29))
  (return false))

(fn ResolveCollision
  (params (pLowPriorityAction :type Action%20Base%20Object%20Reference) (collisionPlacement :type Int%20Point%20Structure%20%28by%20ref%29) (highPrioEntryBehavior :type Integer) (lowPrioEntryBehavior :type Integer))
  (if (Utilities|EqualTiles collisionPlacement (Class|ActionBase|GetExecutorPlacement pLowPriorityAction))
    (Utilities|AddExecutorasVictim pLowPriorityAction
      (:Out
        (return (Utilities|Struct|MakeActionCollisionResolveResult true true (Class|ActionBase|MaxCancellationCounter)))))
    (elif (Math|Conversions|ToBoolean(Integer) (Class|KismetMathLibrary|AndIntInt lowPrioEntryBehavior (|BitmaskLiteral 4)))
      (Utilities|AddExecutorasVictim pLowPriorityAction
        (:Out
          (return (Utilities|Struct|MakeActionCollisionResolveResult true true 0))))
      (else
        (Utilities|IdleActionZeroUsage
          (:Out
            (if (== (Class|ActionBase|GetBehavior pLowPriorityAction) (Class|ActionBase|IdleActionBehavior))
              (Utilities|AddExecutorasVictim pLowPriorityAction
                (:Out
                  _)))
            (return (Utilities|Struct|MakeActionCollisionResolveResult false true 0))))))))

(fn StartTornado
  (bind _mdistribution (Variables|Default|GetmDistribution))
  (bind _returnvalue (Game|SpawnActorfromClass "/Game/Blueprints/BP_Tornado.BP_Tornado_C" (Math|Transform|MakeTransform "0, 0, 0" "0, 0, 0" "1,1,1") "Undefined" 0 0))
  (LocalVariables|SetLTornado _returnvalue)
  (Utilities|FlowControl|Sequence
    (:then_0
      (for _index (range 1 (Utilities|Array|LastIndex _mdistribution))
        (Utilities|Array|Add (LocalVariables|GetLPath) (Class|PassMap|GetTilePositionWorld (Class|ArenaUtilities|GetPassMap) (.mtile (Utilities|Array|Get(acopy) _mdistribution _index))))))
    (:then_1
      (Default|SetPath (LocalVariables|GetLTornado) (LocalVariables|GetLPath))
      (Default|StartTornado (LocalVariables|GetLTornado) (Variables|Default|GetTornadoDuration))
      (return (LocalVariables|GetLTornado)))))

(fn TryDistributeat
  (params (potentialDistributionTile :type Int%20Point%20Structure%20%28by%20ref%29))
  (return (Variables|Default|GetmActionBehavior) true))

(fn CanbeSetupat
  (params (potentialSetupTile :type Int%20Point%20Structure%20%28by%20ref%29))
  (return true))

(fn FinalizeSetupProcess
  (return true))

(fn AffectTargets
  (LocalVariables|SetLBattleLog (Class|ArenaUtilities|GetBattleLog))
  (for _array_element (Variables|Default|GetTargets)
    (bind _returnvalue (Class|BattleLog|CreateBattleLogItemActionAffectsCreature (LocalVariables|GetLBattleLog) self _array_element))
    (Utilities|Array|Add (LocalVariables|GetLBattleLogItems) _returnvalue)
    (Class|Damageable|ExecuteDamageableTask (Class|CreatureBase|GetDamageableComponent _array_element) (Utilities|Struct|MakeDamageableTask "Damage" (Variables|Default|GetDamage) self (Class|ActionBase|GetExecutionPriority) _returnvalue)))
  (Class|BattleLog|PushBattleLogItems (LocalVariables|GetLBattleLog) (LocalVariables|GetLBattleLogItems)))