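; Arena combat action for throwing a stone, which can stun when several throws stack together.
; When it collides with a lower-priority stone throw and entry flags allow, both increment their stack count and the higher-priority one stops being last in stack.
; After collision resolution, an uncanceled last-in-stack throw that reaches the threshold queues a Stun status effect task; other collisions defer to the parent.
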(event Custom|FinishCollisionResolve_Inner
  (if (Math|Boolean|ANDBoolean (not (Variables|Default|GetmIsCanceled)) (Variables|Default|GetLastInStack) (>= (+ (Variables|Default|GetThrowStonesStackSize) 1) (Variables|Default|GetStackSizeToActivateStatusEffect)))
    (Utilities|Array|Add (Variables|Default|GetStatusEffectTasks) (Utilities|Struct|MakeStatusEffectTask "/Game/Blueprints/Arena/StatusEffects/BP_StatusEffect_Stun.BP_StatusEffect_Stun_C" 1 1 0 0))))

(event EventReset
  (|CallParentFunction)
  (Utilities|Array|Clear (Variables|Default|GetStatusEffectTasks)))

(fn ConstructionScript
  (|CallParentFunction))

(fn PowerUp
  (Math|Integer|IncrementInt (Variables|Default|GetThrowStonesStackSize)))

(fn ResolveCollision
  (params (pLowPriorityAction :type Action%20Base%20Object%20Reference) (collisionPlacement :type Int%20Point%20Structure%20%28by%20ref%29) (highPrioEntryBehavior :type Integer) (lowPrioEntryBehavior :type Integer))
  (bind _returnvalue (|BitmaskLiteral 2))
  (bind (_asbp_action_throw_stone _bsuccess) (Utilities|Casting|CastToBP_Action_ThrowStone pLowPriorityAction))
  (if (Math|Boolean|ANDBoolean _bsuccess (not (Math|Conversions|ToBoolean(Integer) (Class|KismetMathLibrary|AndIntInt _returnvalue highPrioEntryBehavior))) (not (Math|Conversions|ToBoolean(Integer) (Class|KismetMathLibrary|AndIntInt _returnvalue lowPrioEntryBehavior))))
    (CallFunction|PowerUp _asbp_action_throw_stone)
    (CallFunction|PowerUp)
    (Variables|Default|SetLastInStack false)
    (return (Utilities|Struct|MakeActionCollisionResolveResult false 0))
    (else
      (bind _returnvalue_2 (|CallParentFunction pLowPriorityAction collisionPlacement highPrioEntryBehavior lowPrioEntryBehavior))
      (return _returnvalue_2))))