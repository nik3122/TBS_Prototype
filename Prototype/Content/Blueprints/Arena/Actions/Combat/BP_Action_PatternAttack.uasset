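; Arena combat action that hits every damageable unit on the tiles of a distribution pattern.
; Distribution collects occupants as targets; pre-execution applies status effect tasks and damage to each, with battle log items for creatures.
; Execution is presentational: the executor aims at the last distributed tile and plays an animation, stopping when it finishes.
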(event EventPreExecutionApply
  (CallFunction|AffectsTargets))

(event EventPostExecutionApply)

(event EventOnStartExecution
  (bind _mdistribution (Variables|Default|GetmDistribution))
  (Class|TiledMovement|AimatTile (Variables|Default|GetmpExecutorTiledMovement) (.mtile (Utilities|Array|Get(acopy) _mdistribution (Utilities|Array|LastIndex _mdistribution))))
  (if (not (Variables|Default|GetmIsCanceled))
    (bind _animationmanager (Utilities|IfExecutorHasAnimationManager)
      (:Is%20Valid
        (bind _returnvalue (Class|AnimationManager|TryPlaySingleActionAnimation _animationmanager (Variables|Action|GetAnimationSectionName)))
        (if _returnvalue
          (EventDispatchers|BindEventtoMEventSingleActionAnimationFinished _animationmanager (EventDispatchers|CreateEvent :!event OnAnimationFinished))
          (else
            (Class|ActionBase|StopExecution)))))))

(event EventReset
  (|CallParentFunction)
  (Utilities|Array|Clear (Variables|Default|GetTargets)))

(event EventOnStopExecution)

(fn ConstructionScript)

(fn TryDistributeat
  (params (potentialDistributionTile :type Int%20Point%20Structure%20%28by%20ref%29))
  (bind _asarena_unit_interface (Utilities|Casting|CastToArenaUnit_Interface (Class|PassMap|GetOccupant (Class|ArenaUtilities|GetPassMap) potentialDistributionTile "OccupationSlot_ArenaUnit"))
    (:then
      (bind _returnvalue (Class|ArenaUnitInterface|GetDamageable _asarena_unit_interface))
      (Utilities|IsValid _returnvalue
        (:Is%20Valid
          (Utilities|Array|Add (Variables|Default|GetTargets) _asarena_unit_interface)
          (return (Variables|Default|GetmActionBehavior) true))
        (:Is%20Not%20Valid
          (return 0 false))))
    (:CastFailed
      (return 0 false))))

(fn CanbeSetupat
  (params (potentialSetupTile :type Int%20Point%20Structure%20%28by%20ref%29))
  (return true))

(fn FinalizeSetupProcess
  (return true))

(fn OnAnimationFinished
  (Class|ActionBase|StopExecution))

(fn AffectsTargets
  (bind _lbattlelogitems (LocalVariables|GetLBattleLogItems))
  (LocalVariables|SetLBattleLog (Class|ArenaUtilities|GetBattleLog))
  (for _array_element (Variables|Default|GetTargets)
    (bind _ascreature_base (Utilities|Casting|CastToCreatureBase _array_element)
      (:then
        (bind _returnvalue (Class|BattleLog|CreateBattleLogItemActionAffectsCreature (LocalVariables|GetLBattleLog) self _ascreature_base))
        (Utilities|Array|Add (LocalVariables|GetLBattleLogItems) _returnvalue)
        (Utilities|FlowControl|Sequence
          (:then_0
            (for _array_element_2 (Variables|Action|GetStatusEffectTasks)
              (bind _structout (Utilities|Struct|SetmembersinStatusEffectTask _array_element_2 (Class|ActionBase|GetExecutionPriority) _returnvalue))
              (Class|StatusEffectsManager|ExecuteStatusEffectTask (Class|CreatureBase|GetStatusEffectsManagerComponent _ascreature_base) _structout)))
          (:then_1
            (Class|Damageable|ExecuteDamageableTask (Class|CreatureBase|GetDamageableComponent _ascreature_base) (Utilities|Struct|MakeDamageableTask "Damage" (Variables|Action|GetDamage) (Class|ActionBase|GetExecutorActor) (Class|ActionBase|GetExecutionPriority) _returnvalue)))))
      (:CastFailed
        (Utilities|FlowControl|Sequence
          (:then_0
            (bind _returnvalue_2 (Class|ArenaUnitInterface|GetStatusEffectsManager _array_element))
            (Utilities|IsValid _returnvalue_2
              (:Is%20Valid
                (for _array_element_3 (Variables|Action|GetStatusEffectTasks)
                  (Class|StatusEffectsManager|ExecuteStatusEffectTask _returnvalue_2 _array_element_3)))))
          (:then_1
            (bind _returnvalue_3 (Class|ArenaUnitInterface|GetDamageable _array_element))
            (Utilities|IsValid _returnvalue_3
              (:Is%20Valid
                (Class|Damageable|ExecuteDamageableTask _returnvalue_3 (Utilities|Struct|MakeDamageableTask "Damage" (Variables|Action|GetDamage) (Class|ActionBase|GetExecutorActor) (Class|ActionBase|GetExecutionPriority) 0)))))))))
  (if (Utilities|Array|IsValidIndex _lbattlelogitems)
    (Class|BattleLog|PushBattleLogItems (LocalVariables|GetLBattleLog) _lbattlelogitems)))