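; Base arena action for ranged weapon attacks on tiles occupied by damageable units.
; Planning rolls a weather-based miss chance, and distribution collects attack targets tagged with that result.
; Unless it misses, pre-execution applies status effects and damage, logging creature hits to the battle log, separately from the visuals.
; Execution equips the weapon and projectile, passes it the targets, aims at the tile and plays the attack animation, stopping when that finishes.
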(event Custom|OnAnimationFinished
  (Class|ActionBase|StopExecution))

(event EventOnStartExecution
  (if (not (Variables|Default|GetmIsCanceled))
    (bind _returnvalue (Class|ArenaUnitInterface|GetWeaponOperator (Class|ActionBase|GetExecutorArenaUnit)))
    (bind _returnvalue_2 (Class|WeaponOperator|SpawnandEquipWeapon _returnvalue (Variables|Action|GetWeaponType)))
    (Class|WeaponBase|LoadProjectile _returnvalue_2 (Variables|Action|GetProjectileType))
    (Class|WeaponOperator|SetAttackTargets _returnvalue (Variables|Default|GetAttackTargets))
    (bind _returnvalue_3 (Class|ArenaUnitInterface|GetTiledMovement (Class|ActionBase|GetExecutorArenaUnit)))
    (Class|TiledMovement|AimatTile _returnvalue_3 (Class|ActionBase|GetPlacement))
    (bind _animationmanager (Utilities|IfExecutorHasAnimationManager)
      (:Is%20Valid
        (bind _returnvalue_4 (Class|AnimationManager|TryPlaySingleActionAnimation _animationmanager (Variables|Action|GetRangeAttackSectionName)))
        (if _returnvalue_4
          (EventDispatchers|BindEventtoMEventSingleActionAnimationFinished _animationmanager (EventDispatchers|CreateEvent :!event Custom|OnAnimationFinished))
          (else
            (Class|ActionBase|StopExecution))))
      (:Is%20Not%20Valid
        (Class|ActionBase|StopExecution)))))

(event EventPrepareforPlanning
  (bind _returnvalue (Class|ArenaManagerInterface|GetWeather (Class|ArenaUtilities|GetArenaManagerInterface)))
  (Variables|Default|SetIsMissing (>= (.mpossibilitytomissrangeattack (Class|Weather|GetWeatherState _returnvalue)) (Math|Random|RandomIntegerinRange 1 100))))

(event EventReset
  (|CallParentFunction)
  (Utilities|Array|Clear (Variables|Default|GetAttackTargets)))

(event EventPreExecutionApply
  (if (not (Variables|Default|GetIsMissing))
    (CallFunction|AffectTargets)))

(event EventPostExecutionApply)

(event EventOnStopExecution
  (bind _animationmanager (Utilities|IfExecutorHasAnimationManager)
    (:Is%20Valid
      (EventDispatchers|UnbindEventfromMEventSingleActionAnimationFinished _animationmanager (EventDispatchers|CreateEvent :!event Custom|OnAnimationFinished)))))

(fn ConstructionScript)

(fn IsPretendingonTile
  (params (tile :type Int%20Point%20Structure%20%28by%20ref%29))
  (return false))

(fn TryDistributeat
  (params (potentialDistributionTile :type Int%20Point%20Structure%20%28by%20ref%29))
  (bind _returnvalue (Class|ArenaUtilities|GetPassMap))
  (bind _returnvalue_2 (Class|PassMap|GetOccupant _returnvalue potentialDistributionTile "OccupationSlot_ArenaUnit"))
  (bind _asarena_unit_interface (Utilities|Casting|CastToArenaUnit_Interface _returnvalue_2)
    (:then
      (bind _returnvalue_3 (Class|ArenaUnitInterface|GetDamageable _asarena_unit_interface))
      (Utilities|IsValid _returnvalue_3
        (:Is%20Valid
          (Utilities|Array|AddUnique (Variables|Default|GetAttackTargets) (Utilities|Struct|MakeWeaponAttackTarget _returnvalue_2 "0.000000,0.000000,0.000000" (Variables|Default|GetIsMissing)))
          (return (Variables|Default|GetmActionBehavior) true))
        (:Is%20Not%20Valid
          (return 0 false))))
    (:CastFailed
      (return 0 false))))

(fn CanbeSetupat
  (params (potentialSetupTile :type Int%20Point%20Structure%20%28by%20ref%29))
  (bind _asarena_unit_interface (Utilities|Casting|CastToArenaUnit_Interface (Class|PassMap|GetOccupant (Class|ArenaUtilities|GetPassMap) potentialSetupTile "OccupationSlot_ArenaUnit"))
    (:then
      (bind _returnvalue (Class|ArenaUnitInterface|GetDamageable _asarena_unit_interface))
      (return (Utilities|IsValid _returnvalue)))
    (:CastFailed
      (return false))))

(fn FinalizeSetupProcess
  (return true))

(fn AffectTargets
  (LocalVariables|SetLBattleLog (Class|ArenaUtilities|GetBattleLog))
  (Utilities|FlowControl|Sequence
    (:then_0
      (for _array_element (Variables|Default|GetAttackTargets)
        (bind _ascreature_base (Utilities|Casting|CastToCreatureBase (.mptargetactor _array_element))
          (:then
            (bind _returnvalue (Class|BattleLog|CreateBattleLogItemActionAffectsCreature (LocalVariables|GetLBattleLog) self _ascreature_base))
            (Utilities|Array|Add (LocalVariables|GetLBattleLogItems) _returnvalue)
            (Utilities|FlowControl|Sequence
              (:then_0
                (for _array_element_2 (Variables|Action|GetStatusEffectTasks)
                  (bind _structout (Utilities|Struct|SetmembersinStatusEffectTask _array_element_2 (Class|ActionBase|GetExecutionPriority) _returnvalue))
                  (Class|StatusEffectsManager|ExecuteStatusEffectTask (Class|CreatureBase|GetStatusEffectsManagerComponent _ascreature_base) _structout)))
              (:then_1
                (Class|Damageable|ExecuteDamageableTask (Class|CreatureBase|GetDamageableComponent _ascreature_base) (Utilities|Struct|MakeDamageableTask "Damage" (Variables|Action|GetDamage) (Class|ActionBase|GetExecutorActor) (Class|ActionBase|GetExecutionPriority) _returnvalue)))))
          (:CastFailed
            (bind _asarena_unit_interface (Utilities|Casting|CastToArenaUnit_Interface (.mptargetactor _array_element)))
            (Utilities|FlowControl|Sequence
              (:then_0
                (bind _returnvalue_2 (Class|ArenaUnitInterface|GetStatusEffectsManager _asarena_unit_interface))
                (Utilities|IsValid _returnvalue_2
                  (:Is%20Valid
                    (for _array_element_3 (Variables|Action|GetStatusEffectTasks)
                      (Class|StatusEffectsManager|ExecuteStatusEffectTask _returnvalue_2 _array_element_3)))))
              (:then_1
                (bind _returnvalue_3 (Class|ArenaUnitInterface|GetDamageable _asarena_unit_interface))
                (Utilities|IsValid _returnvalue_3
                  (:Is%20Valid
                    (Class|Damageable|ExecuteDamageableTask _returnvalue_3 (Utilities|Struct|MakeDamageableTask "Damage" (Variables|Action|GetDamage) (Class|ActionBase|GetExecutorActor) (Class|ActionBase|GetExecutionPriority) 0))))))))))
    (:then_1
      (Class|BattleLog|PushBattleLogItems (LocalVariables|GetLBattleLog) (LocalVariables|GetLBattleLogItems)))))