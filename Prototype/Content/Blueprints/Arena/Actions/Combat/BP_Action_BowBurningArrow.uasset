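; Arena combat action for a burning arrow bow attack that can also target ignitable tiles and set them on fire.
; Setup and distribution accept tiles the fire system reports as ignitable, alongside those the parent logic allows.
; Ignitable tiles the parent rejects are added to the attack targets at their world position.
; After execution, a shot that did not miss ignites its placement tile through the fire system.
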(event EventPostExecutionApply
  (|CallParentFunction)
  (if (not (Variables|Default|GetIsMissing))
    (Class|FireSystem|SetTileonFire (Class|ArenaUtilities|GetFireSystem) (Class|ActionBase|GetPlacement))))

(fn ConstructionScript
  (|CallParentFunction))

(fn CanbeSetupat
  (params (potentialSetupTile :type Int%20Point%20Structure%20%28by%20ref%29))
  (if (Class|FireSystem|IsTileIgnitable (Class|ArenaUtilities|GetFireSystem) potentialSetupTile)
    (return true)
    (else
      (return (|CallParentFunction potentialSetupTile)))))

(fn TryDistributeat
  (params (potentialDistributionTile :type Int%20Point%20Structure%20%28by%20ref%29))
  (bind (_outbehavioratdistributiontile _returnvalue) (|CallParentFunction potentialDistributionTile))
  (if _returnvalue
    (return _outbehavioratdistributiontile true)
    (elif (Class|FireSystem|IsTileIgnitable (Class|ArenaUtilities|GetFireSystem) potentialDistributionTile)
      (Utilities|Array|Add (Variables|Default|GetAttackTargets) (Utilities|Struct|MakeWeaponAttackTarget 0 (Class|PassMap|GetTilePositionWorld (Class|ArenaUtilities|GetPassMap) potentialDistributionTile) (Variables|Default|GetIsMissing)))
      (return (Variables|Default|GetmActionBehavior) true)
      (else
        (return 0 false)))))