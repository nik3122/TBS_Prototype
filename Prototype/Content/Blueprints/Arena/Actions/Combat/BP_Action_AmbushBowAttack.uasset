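; Arena combat action for an ambush bow attack that damages units on its tiles and fires a projectile at each of the executor's enemies.
; Tile distribution gathers damageable occupants as Targets, which take battle-logged damage in pre-execution, separate from projectile launch.
; Projectiles spawn on a circle around the enemies' center of mass, along each enemy's direction.
; Execution stops if the animation cannot play; flagged collisions change the cancellation counter without interrupting.
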(event EventReset
  (|CallParentFunction)
  (Utilities|Array|Clear (Variables|Default|GetTargets)))

(event EventPreExecutionApply
  (CallFunction|AffectTargets))

(event EventOnStopExecution
  (bind _animationmanager (Utilities|IfExecutorHasAnimationManager)
    (:Is%20Valid
      (EventDispatchers|UnbindEventfromMEventSingleActionAnimationFinished _animationmanager (EventDispatchers|CreateEvent :!event StopExecution)))))

(event EventPostExecutionApply)

(event EventOnStartExecution
  (if (not (Variables|Default|GetmIsCanceled))
    (CallFunction|LaunchProjectiles)
    (bind _animationmanager (Utilities|IfExecutorHasAnimationManager)
      (:Is%20Valid
        (bind _returnvalue (Class|AnimationManager|TryPlaySingleActionAnimation _animationmanager (Variables|Default|GetSingleAnimationSection)))
        (if _returnvalue
          (EventDispatchers|BindEventtoMEventSingleActionAnimationFinished _animationmanager (EventDispatchers|CreateEvent :!event StopExecution))
          (else
            (Class|ActionBase|StopExecution))))
      (:Is%20Not%20Valid
        (Class|ActionBase|StopExecution)))))

(fn ConstructionScript)

(fn ResolveCollision
  (params (pLowPriorityAction :type Action%20Base%20Object%20Reference) (collisionPlacement :type Int%20Point%20Structure%20%28by%20ref%29) (highPrioEntryBehavior :type Integer) (lowPrioEntryBehavior :type Integer))
  (if (Math|Conversions|ToBoolean(Integer) (Class|KismetMathLibrary|AndIntInt lowPrioEntryBehavior (|BitmaskLiteral 2)))
    ;[1 1 1] Cancellation counter if colliding with executor.
    (return (Utilities|Struct|MakeActionCollisionResolveResult false (Variables|Default|GetmCancellationCounterChange)))
    (else
      (return (Utilities|Struct|MakeActionCollisionResolveResult false 0)))))

(fn LaunchProjectiles
  (bind _returnvalue (Class|ArenaUnitInterface|GetSocialComponent (Variables|Default|GetmpExecutorUnit)))
  (for _array_element (Class|SocialComponent|GetEnemies _returnvalue)
    (bind _returnvalue_2 (Game|SpawnActorfromClass (Variables|Default|GetProjectileType) (Math|Transform|MakeTransform "0, 0, 0" "0, 0, 0" "1,1,1") "AlwaysSpawn" 0 0))
    ;[1 1 1] Launch target projectile from a random point on the circle of LaunchRadius around enemies center mass.
    (Class|ProjectileBase|LaunchwithTargetActor _returnvalue_2 (+ (* (Math|Vector|Normalize (- (Transformation|GetActorLocation _array_element) (Variables|Default|GetEnemiesCenterMassPosition))) (LocalVariables|GetLLaunchRadius)) (Variables|Default|GetEnemiesCenterMassPosition)) _array_element (Class|ActionBase|GetExecutorActor))))

(fn TryDistributeat
  (params (potentialDistributionTile :type Int%20Point%20Structure%20%28by%20ref%29))
  (bind _asarena_unit_interface (Utilities|Casting|CastToArenaUnit_Interface (Class|PassMap|GetOccupant (Class|ArenaUtilities|GetPassMap) potentialDistributionTile "OccupationSlot_ArenaUnit"))
    (:then
      (bind _returnvalue (Class|ArenaUnitInterface|GetDamageable _asarena_unit_interface))
      (Utilities|IsValid _returnvalue
        (:Is%20Valid
          (Utilities|Array|AddUnique (Variables|Default|GetTargets) _asarena_unit_interface)
          (return (Variables|Default|GetmActionBehavior) true))
        (:Is%20Not%20Valid
          (return 0 false))))
    (:CastFailed
      (return 0 false))))

(fn CanbeSetupat
  (params (potentialSetupTile :type Int%20Point%20Structure%20%28by%20ref%29))
  (return true))

(fn FinalizeSetupProcess
  (return true))

(fn AffectTargets
  (bind _returnvalue (Class|ActionBase|GetExecutionPriority))
  (bind _self self)
  (bind _damage (Variables|Default|GetDamage))
  (LocalVariables|SetLBattleLog (Class|ArenaUtilities|GetBattleLog))
  (for _array_element (Variables|Default|GetTargets)
    (bind _returnvalue_2 (Class|ArenaUnitInterface|GetDamageable _array_element))
    (Utilities|IsValid _returnvalue_2
      (:Is%20Valid
        (bind _ascreature_base (Utilities|Casting|CastToCreatureBase _array_element)
          (:then
            (bind _returnvalue_3 (Class|BattleLog|CreateBattleLogItemActionAffectsCreature (LocalVariables|GetLBattleLog) self _ascreature_base))
            (Class|Damageable|ExecuteDamageableTask _returnvalue_2 (Utilities|Struct|MakeDamageableTask "Damage" _damage _self _returnvalue _returnvalue_3))
            (Utilities|Array|Add (LocalVariables|GetLBattleLogItems) _returnvalue_3))
          (:CastFailed
            (Class|Damageable|ExecuteDamageableTask _returnvalue_2 (Utilities|Struct|MakeDamageableTask "Damage" _damage _self _returnvalue 0)))))))
  (Class|BattleLog|PushBattleLogItems (LocalVariables|GetLBattleLog) (LocalVariables|GetLBattleLogItems)))