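; Arena combat action for a lightning spell that hits damageable units on the tiles it is distributed to.
; Distribution records each victim with its tile distance from the action's placement, which feeds the damage modifier.
; PreExecutionApply damages all victims at once, pushing battle log entries for creatures.
; Execution separately plays the cast animation and spawns Niagara strikes victim by victim at random delays, so visuals are decoupled from damage.
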(event EventReset
  (|CallParentFunction)
  (Utilities|Array|Clear (Variables|Default|GetVictimsInfo))
  (Variables|Default|SetNextVictimIndex 0))

(event EventPreExecutionApply
  (CallFunction|AffectTargets))

(event EventPostExecutionApply)

(event EventOnStartExecution
  (if (not (Variables|Default|GetmIsCanceled))
    (bind _animationmanager (Utilities|IfExecutorHasAnimationManager)
      (:Is%20Valid
        (bind _returnvalue (Class|AnimationManager|TryPlaySingleActionAnimation _animationmanager (Variables|Default|GetActionSectionName)))
        (if _returnvalue
          (EventDispatchers|BindEventtoMEventSingleActionAnimationFinished _animationmanager (EventDispatchers|CreateEvent :!event StopExecution))
          (if (Variables|Default|GetmIsExecuting) :!label _label
            (Utilities|FlowControl|Delay (Math|Random|RandomFloatinRange (Variables|Default|GetDamageDelayMin) (Variables|Default|GetDamageDelayMax)))
            (bind _allvictimsprocessed (CallFunction|ProcessNextVictim))
            (if (not _allvictimsprocessed)
              (goto _label)))
          (else
            (Class|ActionBase|StopExecution :!label _label_2))))
      (:Is%20Not%20Valid
        (goto _label_2)))))

(event EventOnStopExecution
  (bind _animationmanager (Utilities|IfExecutorHasAnimationManager)
    (:Is%20Valid
      (EventDispatchers|UnbindEventfromMEventSingleActionAnimationFinished _animationmanager (EventDispatchers|CreateEvent :!event StopExecution)))))

(fn ConstructionScript)

(fn AffectTargets
  (LocalVariables|SetLBattleLog (Class|ArenaUtilities|GetBattleLog))
  (for _array_element (Variables|Default|GetVictimsInfo)
    (bind _ascreature_base (Utilities|Casting|CastToCreatureBase (.actor _array_element))
      (:then
        (|DamageCreature _ascreature_base (Class|DamageOperator|ModifyDamage (Variables|Default|GetDamageMinDistance) (Utilities|Struct|MakeAttackModifier "(mAbsolute=0,mPhysical=0,mMagical=0,mPoison=0,mFire=0)" (|DamageFromDistance (.distance _array_element))))))
      (:CastFailed
        (|DamageArenaUnit (.actor _array_element) (Class|DamageOperator|ModifyDamage (Variables|Default|GetDamageMinDistance) (Utilities|Struct|MakeAttackModifier "(mAbsolute=0,mPhysical=0,mMagical=0,mPoison=0,mFire=0)" (|DamageFromDistance (.distance _array_element))))))))
  (Class|BattleLog|PushBattleLogItems (LocalVariables|GetLBattleLog) (LocalVariables|GetLBattleLogItems)))

(fn ProcessNextVictim
  (bind _victimsinfo (Variables|Default|GetVictimsInfo))
  (bind _nextvictimindex (Variables|Default|GetNextVictimIndex))
  (bind _output (Utilities|Array|Get(acopy) _victimsinfo _nextvictimindex))
  (if (Utilities|Array|IsValidIndex (Variables|Default|GetVictimsInfo))
    (LocalVariables|SetLVictim (.actor _output))
    (LocalVariables|SetLDistance (.distance _output))
    (Utilities|Array|SetArrayElem _victimsinfo _nextvictimindex (Utilities|Struct|MakeSTRC_LightningVictimData (.actor _output) (.distance _output) true))
    (Niagara|SpawnSystematLocation "/Game/FX/Lightning/NGR_SYS_LightningStrike.NGR_SYS_LightningStrike" (Transformation|GetActorLocation (LocalVariables|GetLVictim)))
    (bind _result (Math|Integer|IncrementInt (Variables|Default|GetNextVictimIndex))
      (:%20%20
        (return (not (Utilities|Array|IsValidIndex (Variables|Default|GetVictimsInfo) _result)))))
    (else
      (return true))))

(fn TryDistributeat
  (params (potentialDistributionTile :type Int%20Point%20Structure%20%28by%20ref%29))
  (bind _returnvalue (Class|ArenaUtilities|GetPassMap))
  (bind _returnvalue_2 (Class|PassMap|GetOccupant _returnvalue potentialDistributionTile "OccupationSlot_ArenaUnit"))
  (bind _asarena_unit_interface (Utilities|Casting|CastToArenaUnit_Interface _returnvalue_2)
    (:then
      (bind _returnvalue_3 (Class|ArenaUnitInterface|GetDamageable _asarena_unit_interface))
      (Utilities|IsValid _returnvalue_3
        (:Is%20Valid
          (Utilities|Array|Add (Variables|Default|GetVictimsInfo) (Utilities|Struct|MakeSTRC_LightningVictimData _returnvalue_2 (Class|PassMap|GetDistance _returnvalue potentialDistributionTile (Class|ActionBase|GetPlacement)) false))
          (return (Variables|Default|GetmActionBehavior) true))
        (:Is%20Not%20Valid
          (return 0 false))))
    (:CastFailed
      (return 0 false))))

(fn CanbeSetupat
  (params (potentialSetupTile :type Int%20Point%20Structure%20%28by%20ref%29))
  (return true))

(fn FinalizeSetupProcess
  (return true))