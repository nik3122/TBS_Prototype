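; Arena action that shields the executing unit with a temporary defence bonus.
; PreExecutionApply sends an AddDefenceBonus task to the unit's Damageable, and PostExecutionApply sends the negated value to undo it, both at the action's execution priority.
; Execution stops as soon as it starts, since the effect lives entirely in those two hooks.
; Setup and distribution accept any tile, and collision resolution adds no logic.
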(event EventOnStopExecution)

(event EventPreExecutionApply
  (bind _returnvalue (Class|ArenaUnitInterface|GetDamageable (Class|ActionBase|GetExecutorArenaUnit)))
  (Class|Damageable|ExecuteDamageableTask _returnvalue (Utilities|Struct|MakeDamageableTask "AddDefenceBonus" (Variables|Default|GetDefenceBonus) self (Class|ActionBase|GetExecutionPriority) 0)))

(event EventPostExecutionApply
  (bind _returnvalue (Class|ArenaUnitInterface|GetDamageable (Class|ActionBase|GetExecutorArenaUnit)))
  (Class|Damageable|ExecuteDamageableTask _returnvalue (Utilities|Struct|MakeDamageableTask "AddDefenceBonus" (Class|DamageOperator|NegateDamage (Variables|Default|GetDefenceBonus)) self (Class|ActionBase|GetExecutionPriority) 0)))

(event EventOnStartExecution
  (Class|ActionBase|StopExecution))

(fn ConstructionScript)

(fn ResolveCollision
  (params (pLowPriorityAction :type Action%20Base%20Object%20Reference) (collisionPlacement :type Int%20Point%20Structure%20%28by%20ref%29) (highPrioEntryBehavior :type Integer) (lowPrioEntryBehavior :type Integer))
  (return ""))

(fn CanbeSetupat
  (params (potentialSetupTile :type Int%20Point%20Structure%20%28by%20ref%29))
  (return true))

(fn TryDistributeat
  (params (potentialDistributionTile :type Int%20Point%20Structure%20%28by%20ref%29))
  (return (Variables|Default|GetmActionBehavior) true))

(fn FinalizeSetupProcess
  (return true))