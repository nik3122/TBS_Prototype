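; Bark arena action that applies one status effect task to allied creatures and another to enemies.
; During distribution, it sorts each tile's occupying creature into Allies or Enemies by party membership with the executor, returning a different behavior flag for each.
; PreExecutionApply runs both status tasks at the action's priority and pushes per-target battle log items; execution itself stops immediately.
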(event EventOnStopExecution)

(event EventPreExecutionApply
  (CallFunction|AffectTargets))

(event EventReset
  (Utilities|Array|Clear (Variables|Default|GetAllies))
  (Utilities|Array|Clear (Variables|Default|GetEnemies))
  (|CallParentFunction))

(event EventPostExecutionApply)

(event EventOnStartExecution
  (Class|ActionBase|StopExecution))

(fn ConstructionScript)

(fn ResolveCollision
  (params (pLowPriorityAction :type Action%20Base%20Object%20Reference) (collisionPlacement :type Int%20Point%20Structure%20%28by%20ref%29) (highPrioEntryBehavior :type Integer) (lowPrioEntryBehavior :type Integer))
  (return ""))

(fn TryDistributeat
  (params (potentialDistributionTile :type Int%20Point%20Structure%20%28by%20ref%29))
  (bind _ascreature_base (Utilities|Casting|CastToCreatureBase (Class|PassMap|GetOccupant (Class|ArenaUtilities|GetPassMap) potentialDistributionTile "OccupationSlot_ArenaUnit"))
    (:then
      (bind _returnvalue (Class|ArenaUnitInterface|GetSocialComponent _ascreature_base))
      (if (.ReturnValue (Class|Party|IsinParty (Class|SocialComponent|GetParty _returnvalue) (.AsCreature%20Base (Utilities|Casting|CastToCreatureBase (Class|ActionBase|GetExecutorActor)))))
        (Utilities|Array|Add (Variables|Default|GetAllies) _ascreature_base)
        (return (|BitmaskLiteral 32) true)
        (else
          (Utilities|Array|Add (Variables|Default|GetEnemies) _ascreature_base)
          (return (|BitmaskLiteral 64) true))))
    (:CastFailed
      (return 0 false))))

(fn CanbeSetupat
  (params (potentialSetupTile :type Int%20Point%20Structure%20%28by%20ref%29))
  (return true))

(fn FinalizeSetupProcess
  (return true))

(fn AffectTargets
  (Utilities|FlowControl|Sequence
    (:then_0
      (for _array_element (Variables|Default|GetAllies)
        (bind _returnvalue (Class|BattleLog|CreateBattleLogItemActionAffectsCreature (Class|ArenaUtilities|GetBattleLog) self _array_element))
        (bind _structout (Utilities|Struct|SetmembersinStatusEffectTask (Variables|Default|GetAllyStatusEffectTasks) (Class|ActionBase|GetExecutionPriority) _returnvalue))
        (Class|StatusEffectsManager|ExecuteStatusEffectTask (Class|CreatureBase|GetStatusEffectsManagerComponent _array_element) _structout)
        (Utilities|Array|Add (LocalVariables|GetLBattleLogItems) _returnvalue)))
    (:then_1
      (for _array_element_2 (Variables|Default|GetEnemies)
        (bind _returnvalue_2 (Class|BattleLog|CreateBattleLogItemActionAffectsCreature (Class|ArenaUtilities|GetBattleLog) self _array_element_2))
        (bind _structout_2 (Utilities|Struct|SetmembersinStatusEffectTask (Variables|Default|GetEnemyStatusEffectTasks) (Class|ActionBase|GetExecutionPriority) _returnvalue_2))
        (Class|StatusEffectsManager|ExecuteStatusEffectTask (Class|CreatureBase|GetStatusEffectsManagerComponent _array_element_2) _structout_2)
        (Utilities|Array|Add (LocalVariables|GetLBattleLogItems) _returnvalue_2)))
    (:then_2
      (Class|BattleLog|PushBattleLogItems (Class|ArenaUtilities|GetBattleLog) (LocalVariables|GetLBattleLogItems)))))