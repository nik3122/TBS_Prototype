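; Horn of Heroes is an arena buff/debuff action that applies a status effect task to every creature on the tiles it is distributed to.
; Distribution collects tile occupants as targets, then pre-execution runs the task on each at the action's priority and pushes battle log entries.
; Execution, unless canceled, plays a single-action animation and binds to its finish event, stopping immediately if no animation can play.
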(event EventOnStopExecution
  (bind _animationmanager (Utilities|IfExecutorHasAnimationManager)
    (:Is%20Valid
      (EventDispatchers|UnbindEventfromMEventSingleActionAnimationFinished _animationmanager (EventDispatchers|CreateEvent :!event StopExecution)))))

(event EventPreExecutionApply
  (CallFunction|AffectTargets))

(event EventReset
  (Utilities|Array|Clear (Variables|Default|GetTargets))
  (|CallParentFunction))

(event EventPostExecutionApply)

(event EventOnStartExecution
  (if (not (Variables|Default|GetmIsCanceled))
    (bind _animationmanager (Utilities|IfExecutorHasAnimationManager)
      (:Is%20Valid
        (bind _returnvalue (Class|AnimationManager|TryPlaySingleActionAnimation _animationmanager (Variables|Default|GetSingleActionAnimSection)))
        (if _returnvalue
          (EventDispatchers|BindEventtoMEventSingleActionAnimationFinished _animationmanager (EventDispatchers|CreateEvent :!event StopExecution))
          (else
            (Class|ActionBase|StopExecution))))
      (:Is%20Not%20Valid
        (Class|ActionBase|StopExecution)))))

(fn ConstructionScript)

(fn ResolveCollision
  (params (pLowPriorityAction :type Action%20Base%20Object%20Reference) (collisionPlacement :type Int%20Point%20Structure%20%28by%20ref%29) (highPrioEntryBehavior :type Integer) (lowPrioEntryBehavior :type Integer))
  (return (Utilities|Struct|MakeActionCollisionResolveResult false 0)))

(fn TryDistributeat
  (params (potentialDistributionTile :type Int%20Point%20Structure%20%28by%20ref%29))
  (bind _ascreature_base (Utilities|Casting|CastToCreatureBase (Class|PassMap|GetOccupant (Class|ArenaUtilities|GetPassMap) potentialDistributionTile "OccupationSlot_ArenaUnit"))
    (:then
      (Utilities|Array|Add (Variables|Default|GetTargets) _ascreature_base)
      (return (Variables|Default|GetmActionBehavior) true))
    (:CastFailed
      (return 0 false))))

(fn CanbeSetupat
  (params (potentialSetupTile :type Int%20Point%20Structure%20%28by%20ref%29))
  (return true))

(fn FinalizeSetupProcess
  (return true))

(fn AffectTargets
  (Utilities|FlowControl|Sequence
    (:then_0
      (for _array_element (Variables|Default|GetTargets)
        (bind _returnvalue (Class|BattleLog|CreateBattleLogItemActionAffectsCreature (Class|ArenaUtilities|GetBattleLog) self _array_element))
        (Utilities|Array|Add (LocalVariables|GetLBattleLogItems) _returnvalue)
        (bind _structout (Utilities|Struct|SetmembersinStatusEffectTask (Variables|Default|GetStatusEffectTask) (Class|ActionBase|GetExecutionPriority) _returnvalue))
        (Class|StatusEffectsManager|ExecuteStatusEffectTask (Class|CreatureBase|GetStatusEffectsManagerComponent _array_element) _structout)))
    (:then_1
      (Class|BattleLog|PushBattleLogItems (Class|ArenaUtilities|GetBattleLog) (LocalVariables|GetLBattleLogItems)))))