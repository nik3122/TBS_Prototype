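; Arena action Ancient Roots: spawns a roots effect over its distributed tiles and damages units whose lower-priority actions collide with it.
; ResolveCollision interrupts actions with matching behavior bits and collects their executors' damageables, which take damage in PreExecutionApply, with battle log entries for creatures.
; On execution, the executor aims at the placement, BP_AncientRoots receives every tile position except the first, and a single-action animation plays, stopping execution if unavailable.
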(event EventPreExecutionApply
  (bind _returnvalue (Class|ArenaUtilities|GetBattleLog))
  (for _array_element (Variables|Default|GetTargetDamageables)
    (bind _asbp_creature_base (Utilities|Casting|CastToBP_Creature_Base (Components|GetOwner _array_element))
      (:then
        (bind _returnvalue_2 (Class|BattleLog|CreateBattleLogItemActionAffectsCreature _returnvalue self _asbp_creature_base))
        (Class|Damageable|ExecuteDamageableTask _array_element (Utilities|Struct|MakeDamageableTask "Damage" (Variables|Default|GetDamage) self (Class|ActionBase|GetExecutionPriority) _returnvalue_2))
        (Class|BattleLog|PushBattleLogItem _returnvalue _returnvalue_2))
      (:CastFailed
        (Class|Damageable|ExecuteDamageableTask _array_element (Utilities|Struct|MakeDamageableTask "Damage" (Variables|Default|GetDamage) self (Class|ActionBase|GetExecutionPriority) 0))))))

(event EventReset
  (|CallParentFunction)
  (Utilities|Array|Clear (Variables|Default|GetTargetDamageables)))

(event EventPostExecutionApply)

(event EventOnStopExecution
  (bind _animationmanager (Utilities|IfExecutorHasAnimationManager)
    (:Is%20Valid
      (EventDispatchers|UnbindEventfromMEventSingleActionAnimationFinished _animationmanager (EventDispatchers|CreateEvent :!event StopExecution)))))

(event EventOnStartExecution
  (Class|TiledMovement|AimatTile (Class|ActionBase|GetExecutorTiledMovement) (Class|ActionBase|GetPlacement))
  (if (not (Variables|Default|GetmIsCanceled))
    (CallFunction|LaunchFX)
    (bind _animationmanager (Utilities|IfExecutorHasAnimationManager)
      (:Is%20Valid
        (bind _returnvalue (Class|AnimationManager|TryPlaySingleActionAnimation _animationmanager (Variables|Default|GetSingleActionAnimSectionName)))
        (if _returnvalue
          (EventDispatchers|BindEventtoMEventSingleActionAnimationFinished _animationmanager (EventDispatchers|CreateEvent :!event StopExecution))
          (else
            (Class|ActionBase|StopExecution))))
      (:Is%20Not%20Valid
        (Class|ActionBase|StopExecution)))))

(fn ConstructionScript)

(fn ResolveCollision
  (params (pLowPriorityAction :type Action%20Base%20Object%20Reference) (collisionPlacement :type Int%20Point%20Structure%20%28by%20ref%29) (highPrioEntryBehavior :type Integer) (lowPrioEntryBehavior :type Integer))
  (if (Math|Conversions|ToBoolean(Integer) (Class|KismetMathLibrary|AndIntInt lowPrioEntryBehavior (|BitmaskLiteral 6)))
    (bind _returnvalue (Class|ArenaUnitInterface|GetDamageable (Class|ActionBase|GetExecutorArenaUnit pLowPriorityAction)))
    (Utilities|Array|AddUnique (Variables|Default|GetTargetDamageables) _returnvalue)
    (return (Utilities|Struct|MakeActionCollisionResolveResult true 0))
    (else
      (return (Utilities|Struct|MakeActionCollisionResolveResult false 0)))))

(fn LaunchFX
  (Utilities|FlowControl|Sequence
    (:then_0
      (for _index (range 1 (Utilities|Array|LastIndex (Variables|Default|GetmDistribution)))
        (Utilities|Array|Add (LocalVariables|GetLTilesPositions) (Class|PassMap|GetTilePositionWorld (Class|ArenaUtilities|GetPassMap) (.mtile (Utilities|Array|Get(acopy) (Variables|Default|GetmDistribution) _index))))))
    (:then_1
      (Game|SpawnActorfromClass "/Game/FX/AncientRoots/BP_AncientRoots.BP_AncientRoots_C" (Math|Transform|MakeTransform "0, 0, 0" "0, 0, 0" "1,1,1") "AlwaysSpawn" 0 0.15 (LocalVariables|GetLTilesPositions) 3.0 0))))

(fn TryDistributeat
  (params (potentialDistributionTile :type Int%20Point%20Structure%20%28by%20ref%29))
  (return (Variables|Default|GetmActionBehavior) true))

(fn CanbeSetupat
  (params (potentialSetupTile :type Int%20Point%20Structure%20%28by%20ref%29))
  (return true))

(fn FinalizeSetupProcess
  (return true))