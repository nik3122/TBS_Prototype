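; Base weapon Blueprint for the arena, providing shared targeting and projectile-launch helpers, with no active event logic of its own.
; GetTileAnyway resolves a target tile from the victim's TiledMovement component, falls back to the input tile when no victim is valid, and reports failure when the victim lacks that component.
; Launch position and orientation come from the ProjectileLaunchPoint component's world transform.
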(event EventBeginPlay)

(event Collision|EventActorBeginOverlap
  (params (OtherActor :type Actor%20Object%20Reference)))

(event EventTick
  (params (DeltaSeconds :type Float%20%28single-precision%29)))

(fn ConstructionScript)

(fn GetTileAnyway
  (params (Victim :type Actor%20Object%20Reference) (InputTile :type Int%20Point%20Structure))
  (bind _returnvalue (Actor|GetComponentbyClass Victim "/Script/Prototype.TiledMovement"))
  (Utilities|IsValid Victim
    (:Is%20Valid
      (Utilities|IsValid _returnvalue
        (:Is%20Valid
          (return (Class|TiledMovement|GetCurrentTile _returnvalue) true))
        (:Is%20Not%20Valid
          (return "" false))))
    (:Is%20Not%20Valid
      (return InputTile true))))

(fn GetLaunchPosition
  (return (Transformation|GetWorldLocation (Variables|Default|GetProjectileLaunchPoint))))

(fn GetLaunchOrientation
  (return (Transformation|GetWorldRotation (Variables|Default|GetProjectileLaunchPoint))))