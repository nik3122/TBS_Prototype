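; Player controller for the arena lobby that creates and manages the local player's lobby HUD widget.
; BeginPlay polls on a short delay until the player state and arena lobby game state are valid, then calls CreateUI.
; CreateUI spawns the HUD only for a local, non-dedicated-server controller, passing in itself and the game state.
; EndPlay removes the widget from its parent.
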(event EventBeginPlay
  ;[1 0.7637 0] HACK: loop until both game state and player state are valid
  (Utilities|IsValid (Variables|Default|GetPlayerState) :!label _label
    (:Is%20Valid
      (Utilities|Casting|CastToGameState_ArenaLobby (Game|GetGameState)
        (:then
          (CallFunction|CreateUI))
        (:CastFailed
          (Utilities|FlowControl|Delay 0.1 :!label _label_2)
          (goto _label))))
    (:Is%20Not%20Valid
      (goto _label_2))))

(event EventEndPlay
  (params (EndPlayReason :type EEndPlayReason%20Enum :default "Destroyed"))
  (Utilities|IsValid (Variables|Default|GetWidgetHUD)
    (:Is%20Valid
      (Widget|RemovefromParent (Variables|Default|GetWidgetHUD)))))

(fn ConstructionScript)

(fn CreateUI
  (bind _self self)
  (if (and (Pawn|IsLocalPlayerController) (not (Networking|IsDedicatedServer)))
    (bind _returnvalue (UserInterface|CreateWidget "/Game/UI/ArenaLobby/UI_HUD_ArenaLobby.UI_HUD_ArenaLobby_C" _self _self (.AsGame%20State%20Arena%20Lobby (Utilities|Casting|CastToGameState_ArenaLobby (Game|GetGameState)))))
    (bind _output_get (Variables|Default|SetWidgetHUD _returnvalue))
    (UserInterface|Viewport|AddtoViewport _output_get 0)))