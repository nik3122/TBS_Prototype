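; BP_Tornado is a tornado effect actor that moves a particle system along a spline path, then removes itself.
; SetPath supplies the spline points in local space, and StartTornado converts a travel duration into a normalized speed and activates the particles.
; Tick advances normalized time and samples the spline at constant velocity.
; At the path's end it deactivates the particles and destroys the actor after a short delay.
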(event EventBeginPlay)

(event EventTick
  (params (DeltaSeconds :type Float%20%28single-precision%29))
  (if (not (Variables|Default|GetIsFinished))
    (if (<= 1.0 (Variables|Default|GetTime))
      (Variables|Default|SetIsFinished true)
      (Components|Activation|Deactivate (Variables|Default|GetParticleSystem))
      (Utilities|FlowControl|Delay 1.0)
      (Actor|DestroyActor)
      (else
        (Transformation|SetWorldLocation (Variables|Default|GetParticleSystem) (Spline|GetLocationatTime (Variables|Default|GetSpline) (Variables|Default|GetTime) "World" true) false false)
        (Variables|Default|SetTime (+ (Variables|Default|GetTime) (* DeltaSeconds (Variables|Default|GetTimeSpeed))))))))

(fn ConstructionScript)

(fn SetPath
  (params (ControlPoints :type Array%20of%20Vectors))
  (Spline|SetSplinePoints (Variables|Default|GetSpline) ControlPoints "Local" true))

(fn StartTornado
  (params (Time :type Float%20%28single-precision%29))
  (Variables|Default|SetTimeSpeed (/ 1.0 Time))
  (Variables|Default|SetTime 0.0)
  (Variables|Default|SetIsFinished false)
  (Components|Activation|Activate (Variables|Default|GetParticleSystem) true))